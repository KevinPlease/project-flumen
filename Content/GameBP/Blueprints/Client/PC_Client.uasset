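; PC_Client is the client player controller that opens the main menu and external login UI when play begins.
; It creates the WB_MainMenu widget, adds it to the viewport and sets UI-only input without mouse lock.
; Login success and failure both only cast the game instance to GI_Core, as the PlayFab connection call is disconnected for editor testing.
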(event `self.ReceiveBeginPlay`
  ;[0.5417 0.01128 0.01128] TODO: Disabled playfab connection for testing in editor
  (`self.Event Show Main Menu`)
  (`ShowLoginUICallbackProxy.ShowExternalLoginUI` self
    (:`OnSuccess`
      _)
    (:`OnFailure`
      _))
  (bind _asgi_core (cast `/Game/GameBP/Blueprints/GI_Core` (`GameplayStatics.GetGameInstance`))))

(event `Event Show Main Menu`
  (bind _returnvalue (`|CreateWidget` "/Game/GameBP/Blueprints/Client/UI/WB_MainMenu.WB_MainMenu_C" self))
  (bind _output_get (set `self.WB_MainMenu` _returnvalue))
  (`UserWidget.AddToViewport` _output_get 0)
  (`WidgetBlueprintLibrary.SetInputMode_UIOnlyEx` self null))

(fn `UserConstructionScript`)