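; PC_Lobby is the lobby player controller, which puts the main menu on screen for the local player.
; On BeginPlay it calls the gameplay HUD event, which creates and stores WB_MainMenu and adds it to the viewport, then opens the external login UI.
; Login success and failure both lead to a GI_Core cast, but the PlayFab connection call is left unwired, marked as disabled for editor testing.
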(event `self.ReceiveBeginPlay`
  ;[0.5417 0.01128 0.01128] TODO: Disabled playfab connection for testing in editor
  (if (`self.IsLocalController`)
    (`self.Event Show Gameplay HUD`)
    (`ShowLoginUICallbackProxy.ShowExternalLoginUI` self
      (:`OnSuccess`
        _)
      (:`OnFailure`
        _))
    (bind _asgi_core (cast `/Game/GameBP/Blueprints/GI_Core` (`GameplayStatics.GetGameInstance`)))))

(event `Event Show Gameplay HUD`
  (bind _returnvalue (`|CreateWidget` "/Game/GameBP/Blueprints/Gameplay/UI/WB_MainMenu.WB_MainMenu_C" self))
  (bind _output_get (set `self.WB_MainMenu` _returnvalue))
  (`UserWidget.AddToViewport` _output_get 0))

(fn `UserConstructionScript`)