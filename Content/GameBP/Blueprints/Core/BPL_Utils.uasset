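; Blueprint function library of general utilities: Android detection, server joining, match result mapping, PlayFab error reporting and random value generation.
; Join helpers run the "open" console command with an IP and optional port.
; RankToResult converts placement and player count into a result enum, with special rank codes.
; Random generators build numbers or mixed-case strings character by character, clamped to nine characters.
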(fn `GetRandomNumber`
  (params (NumDigits :type Integer))
  (returns (Number :type Integer))
  (locals (RandomNr :type String))
  (for _index (range 1 (+ (`KismetMathLibrary.Clamp` NumDigits 1 9) 1))
    (set `local.RandomNr` (`KismetStringLibrary.Concat_StrStr` (`local.RandomNr`) (`KismetStringLibrary.Conv_IntToString` (select `bool` (== _index 1) :`false` (`KismetMathLibrary.RandomIntegerInRange` 0 9) :`true` (`KismetMathLibrary.RandomIntegerInRange` 1 9))))))
  (return (`KismetStringLibrary.Conv_StringToInt` (`local.RandomNr`))))

(fn `GetRandomString`
  (params (Length :type Integer))
  (returns (GeneratedString :type String))
  (locals (CharsUsed :type "Array of String") (CurString :type String))
  (bind _charsused (`local.CharsUsed`))
  (bind _output (`|GetArrayItem` _charsused (`KismetMathLibrary.RandomIntegerInRange` 1 (`KismetArrayLibrary.Array_LastIndex` _charsused))))
  (for _ (range 1 (+ (`KismetMathLibrary.Clamp` Length 1 9) 1))
    (set `local.CurString` (`KismetStringLibrary.Concat_StrStr` (`local.CurString`) (`KismetMathLibrary.SelectString` (`KismetStringLibrary.ToUpper` _output) _output (`KismetMathLibrary.RandomBool`)))))
  (return (`local.CurString`)))

(fn `HandlePlayFabError`
  (params (PlayFabError :type "PlayFabError Structure (by ref)"))
  (returns (ErrorMsg :type String))
  (bind _returnvalue (`KismetStringLibrary.Concat_StrStr` "Error with PlayFab: " (`.ErrorMessage` (break `PlayFabError` PlayFabError))))
  (`KismetSystemLibrary.PrintString` null _returnvalue)
  (return _returnvalue))

(fn `IsAndroid`
  (returns (IsAndroid :type Boolean))
  (return (== (`GameplayStatics.GetPlatformName`) "Android")))

(fn `JoinServer`
  (params (SpecificPlayer :type "PlayerController Object Reference") (IP :type String) (Port :type Integer))
  (`KismetSystemLibrary.ExecuteConsoleCommand` SpecificPlayer (`KismetTextLibrary.Conv_TextToString` (`|FormatText` "open {IP}:{PORT}" IP (`KismetStringLibrary.Conv_IntToString` Port))) SpecificPlayer))

(fn `JoinServerFullIp`
  (params (SpecificPlayer :type "PlayerController Object Reference") (IP :type String))
  (`KismetSystemLibrary.ExecuteConsoleCommand` SpecificPlayer (`KismetTextLibrary.Conv_TextToString` (`|FormatText` "open {IP}" IP)) SpecificPlayer))

(fn `RankToResult`
  (params (ResultRank :type Integer) (PlayerCount :type Integer))
  (returns (GameResult :type "/Game/GameData/Data/Enums/E_GameResults Enum"))
  (locals (Difference :type Integer) (Result :type "/Game/GameData/Data/Enums/E_GameResults Enum"))
  (if (== ResultRank -1)
    (set `local.Result` "NewEnumerator5")
    (else
      (set `local.Difference` (- PlayerCount ResultRank))
      (if (or (== ResultRank PlayerCount) (== ResultRank -5))
        (set `local.Result` "NewEnumerator2")
        (elif (== ResultRank 1)
          (set `local.Result` "NewEnumerator0")
          (elif (== (`local.Difference`) 1)
            (set `local.Result` "NewEnumerator4")
            (else
              (set `local.Result` "NewEnumerator1")))))))
  (return (`local.Result`)))