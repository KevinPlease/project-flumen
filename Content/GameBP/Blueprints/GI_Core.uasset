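; Game instance for a card and board game client that holds the player profile, save data, themes and audio options across levels.
; On init it loads or creates the save game and fills card and board theme arrays from data tables.
; It builds the profile object from PlayFab info plus saved avatar and settings, saving changes asynchronously.
; Helpers cache the client controller, apply volumes through sound mix overrides and open maps.
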(event `self.ReceiveInit`
  (bind _savegame (`self.LoadSaveGame`))
  (set `self.SaveGameInst` _savegame)
  (`self.Load All Themes`))

(event `Event Create Profile From Playfab Info`
  (params (`Player Profile Playfab Id` :type String) (EntityId :type String) (`Player Profile Display Name` :type String))
  (bind (_playerprofile_playfabid _playerprofile_displayname _playerprofile_avatar _playerprofile_settings) (break `/Game/GameData/Data/Player/ST_PlayerProfile` (`/Game/GameBP/Blueprints/BP_MainSaveGame.PlayerProfile` (`self.SaveGameInst`))))
  (`self.CreateProfile` (make `/Game/GameData/Data/Player/ST_PlayerProfile` `Player Profile Playfab Id` `Player Profile Display Name` _playerprofile_avatar _playerprofile_settings (struct) (`|GetArrayItem` (`self.BoardThemes`)) (`|GetArrayItem` (`self.CardThemes`))))
  (`/Game/GameBP/Blueprints/ClientMenu/Objects/O_PlayerProfile.SetEntityId` (`self.PlayerProfile`) EntityId))

(event `Event Save Profile`
  (bind _savegameinst (`self.SaveGameInst`))
  (`/Game/GameBP/Blueprints/BP_MainSaveGame.Event Save Profile` _savegameinst (`/Game/GameBP/Blueprints/ClientMenu/Objects/O_PlayerProfile.GetPlayerData` (`self.PlayerProfile`)))
  (`AsyncActionHandleSaveGame.AsyncSaveGameToSlot` _savegameinst (`self.PlayerProfileSave`)))

(event `Event Save Profile Options`
  (params (NewOptions :type "/Game/GameData/Data/Player/ST_Options Structure"))
  (set `/Game/GameBP/Blueprints/ClientMenu/Objects/O_PlayerProfile.OptionsData` NewOptions (`self.PlayerProfile`))
  (`self.Event Save Profile`))

(fn `CreateProfile`
  (params (PlayerProfile :type "/Game/GameData/Data/Player/ST_PlayerProfile Structure"))
  (bind _returnvalue (`|GenericCreateObject` "/Game/GameBP/Blueprints/ClientMenu/Objects/O_PlayerProfile.O_PlayerProfile_C" self))
  (bind _profile (`/Game/GameBP/Blueprints/ClientMenu/Objects/O_PlayerProfile.CreateWithData` _returnvalue PlayerProfile))
  (set `self.PlayerProfile` _profile))

(fn `GetPlayerController`
  (returns (PlayerControllerRef :type "/Game/GameBP/Blueprints/ClientMenu/PC_Client Object Reference"))
  (`/Engine/EditorBlueprintResources/StandardMacros.IsValid` (`self.PlayerControllerRef`)
    (:`Is Valid`
      _)
    (:`Is Not Valid`
      (bind _aspc_client (cast `/Game/GameBP/Blueprints/ClientMenu/PC_Client` (`GameplayStatics.GetPlayerController` 0)))
      (set `self.PlayerControllerRef` _aspc_client)))
  (return (`self.PlayerControllerRef`)))

(fn `Load All Themes`
  (`|ExecutionSequence`
    (:`then_0`
      (bind _outrownames (`DataTableFunctionLibrary.GetDataTableRowNames` "/Game/GameData/Data/Gameplay/Theme/DT_CardThemes.DT_CardThemes"))
      (for _array_element _outrownames
        (bind _returnvalue (`|GetDataTableRow` "/Game/GameData/Data/Gameplay/Theme/DT_CardThemes.DT_CardThemes" _array_element)
          (:`then`
            (`KismetArrayLibrary.Array_Add` (`self.CardThemes`) _returnvalue)))))
    (:`then_1`
      (bind _outrownames_2 (`DataTableFunctionLibrary.GetDataTableRowNames` "/Game/GameData/Data/Gameplay/Theme/DT_BoardThemes.DT_BoardThemes"))
      (for _array_element_2 _outrownames_2
        (bind _returnvalue_2 (`|GetDataTableRow` "/Game/GameData/Data/Gameplay/Theme/DT_BoardThemes.DT_BoardThemes" _array_element_2)
          (:`then`
            (`KismetArrayLibrary.Array_Add` (`self.BoardThemes`) _returnvalue_2)))))))

(fn `LoadClientMap`
  (`GameplayStatics.OpenLevel` (`self.ClientMainMap`)))

(fn `LoadOptions`
  (bind (_optionsdata_mastervolume _optionsdata_musicvolume _optionsdata_sfxvolume _optionsdata_uivolume) (break `/Game/GameData/Data/Player/ST_Options` (`/Game/GameBP/Blueprints/ClientMenu/Objects/O_PlayerProfile.OptionsData` (`self.PlayerProfile`))))
  (`self.SetVolume` "NewEnumerator4" _optionsdata_mastervolume)
  (`self.SetVolume` "NewEnumerator0" _optionsdata_musicvolume)
  (`self.SetVolume` "NewEnumerator1" _optionsdata_sfxvolume)
  (`self.SetVolume` "NewEnumerator7" _optionsdata_uivolume))

(fn `LoadSaveGame`
  (returns (SaveGame :type "/Game/GameBP/Blueprints/BP_MainSaveGame Object Reference"))
  (locals (MainSaveGameInst :type "/Game/GameBP/Blueprints/BP_MainSaveGame Object Reference"))
  (bind _returnvalue (`GameplayStatics.DoesSaveGameExist` (`self.PlayerProfileSave`)))
  (if _returnvalue
    (bind _returnvalue_2 (`GameplayStatics.LoadGameFromSlot` (`self.PlayerProfileSave`)))
    (bind _asbp_main_save_game (cast `/Game/GameBP/Blueprints/BP_MainSaveGame` _returnvalue_2))
    (set `local.MainSaveGameInst` _asbp_main_save_game)
    (else
      (bind _returnvalue_3 (`GameplayStatics.CreateSaveGameObject` "/Game/GameBP/Blueprints/BP_MainSaveGame.BP_MainSaveGame_C"))
      (set `local.MainSaveGameInst` _returnvalue_3)))
  (return (`local.MainSaveGameInst`)))

(fn `LoadSingleplayerMap`
  (`GameplayStatics.OpenLevel` (`self.GameplayMap_SP`)))

(fn `SetVolume`
  (params (AudioType :type "/Game/GameData/Data/Enums/E_AudioTypes Enum" :default "NewEnumerator4") (Amount :type "Float (double-precision)"))
  (locals (SoundClass :type "SoundClass Object Reference"))
  (switch `/Game/GameData/Data/Enums/E_AudioTypes` AudioType
    (:`NewEnumerator4`
      (set `local.SoundClass` "/Game/GameBP/Blueprints/Core/Effects/SFX/SC_Master.SC_Master"))
    (:`NewEnumerator0`
      (set `local.SoundClass` "/Game/GameBP/Blueprints/Core/Effects/SFX/SC_Music.SC_Music"))
    (:`NewEnumerator1`
      (set `local.SoundClass` "/Game/GameBP/Blueprints/Core/Effects/SFX/SC_Sfx.SC_Sfx"))
    (:`NewEnumerator7`
      (set `local.SoundClass` "/Game/GameBP/Blueprints/Core/Effects/SFX/SC_UI.SC_UI")))
  (`GameplayStatics.SetSoundMixClassOverride` "/Game/GameBP/Blueprints/Core/Effects/SFX/SM_MasterMix.SM_MasterMix" (`local.SoundClass`) Amount 1.0 0.2))