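; Game mode for the client connect screen that logs the player into PlayFab and loads their profile before entering the client map.
; BeginPlay shows a status widget and logs in by Android device ID, or through iOS login with a test ID on other platforms.
; Success fills the GI_Core profile, pauses for new accounts, then fetches coins via CloudScript and opens MapClient.
; PlayFab failures appear as errors on the widget.
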(event `self.ReceiveBeginPlay`
  ;[1 1 1] Begin Play
  (bind _asgi_core (cast `/Game/GameBP/Blueprints/GI_Core` (`GameplayStatics.GetGameInstance`)))
  (set `self.GameInstancRef` _asgi_core)
  (bind _returnvalue (`|CreateWidget` "/Game/GameBP/Blueprints/ClientConnect/UI/WB_Connect.WB_Connect_C"))
  (bind _output_get (set `self.WB_ClientConnect` _returnvalue))
  (`UserWidget.AddToViewport` _output_get 0)
  (`self.Connect to PlayFab`))

(event `OnSuccess: ConnectService`
  (params (result :type "ClientLoginResult Structure") (customData :type "Object Object Reference"))
  (bind (_entitytoken _inforesultpayload _lastlogintime _newlycreated _playfabid) (break `ClientLoginResult` result))
  ;[1 1 1] Login to Playfab - Create Profile
  (`self.DEBUG_LogOnHUD` "Connected to PlayFab")
  (`/Game/GameBP/Blueprints/GI_Core.Event Create Profile From Playfab Info` (`self.GameInstancRef`) _playfabid (`PlayFabJsonObject.GetStringField` (`PlayFabJsonObject.GetObjectField` _entitytoken "Entity") "Id") (`self.GetNameFromPayload` _inforesultpayload))
  (if _newlycreated
    (`KismetSystemLibrary.Delay` 2.0 :!pinned true) ; TODO: first time players - wait for server to finish adding default data/coins
  )
  (`self.Event Load Player Coins`))

(event `Connect to PlayFab`
  (bind _returnvalue (`MobilePatchingLibrary.GetActiveDeviceProfileName`))
  ;[1 1 1] Login to Playfab - Create Profile
  (if (`/Game/GameBP/Blueprints/BPL_Utils.IsAndroid`)
    (`PlayFabClientAPI.LoginWithAndroidDeviceID` (make `ClientLoginWithAndroidDeviceIDRequest` _returnvalue (`MobileUtilsBlueprintLibrary.GetDeviceId`) true) (delegate `OnSuccess: ConnectService`) (delegate `OnFail: ConnectService`))
    (else
      (`PlayFabClientAPI.LoginWithIOSDeviceID` (make `ClientLoginWithIOSDeviceIDRequest` true null (`self.TEST_RedmiDeviceId`) _returnvalue) (delegate `OnSuccess: ConnectService`) (delegate `OnFail: ConnectService`)))))

(event `OnFail: ConnectService`
  (params (error :type "PlayFabError Structure") (customData :type "Object Object Reference"))
  ;[1 1 1] Login to Playfab - Create Profile
  (bind _errormsg (`/Game/GameBP/Blueprints/BPL_Utils.HandlePlayFabError` error))
  (`self.DEBUG_LogOnHUD` _errormsg true))

(event `OnSuccess: GetPlayerCoins`
  (params (result :type "ClientExecuteCloudScriptResult Structure") (customData :type "Object Object Reference"))
  ;[1 1 1] Load player economy data -- Coins and Update Profile
  (`/Game/GameBP/Blueprints/ClientMenu/Objects/O_PlayerProfile.SetCoins` (`/Game/GameBP/Blueprints/GI_Core.PlayerProfile` (`self.GameInstancRef`)) (`KismetMathLibrary.FTrunc` (`PlayFabJsonValue.AsNumber` (`PlayFabJsonObject.GetField` (`.FunctionResult` (break `ClientExecuteCloudScriptResult` result)) "Value"))))
  (`GameplayStatics.OpenLevel` (`self.MapClient`)))

(event `Event Load Player Coins`
  ;[1 1 1] Load player economy data -- Coins and Update Profile
  (`PlayFabClientAPI.ExecuteCloudScript` (make `ClientExecuteCloudScriptRequest` null "getCoinsForPlayer") (delegate `OnSuccess: GetPlayerCoins`) (delegate `OnFailure: GetPlayerCoins`)))

(event `OnFailure: GetPlayerCoins`
  (params (error :type "PlayFabError Structure") (customData :type "Object Object Reference"))
  ;[1 1 1] Load player economy data -- Coins and Update Profile
  (bind _errormsg (`/Game/GameBP/Blueprints/BPL_Utils.HandlePlayFabError` error))
  (`self.DEBUG_LogOnHUD` _errormsg true))

(fn `DEBUG_LogOnHUD`
  (params (Message :type String) (IsError :type Boolean))
  (bind _wb_clientconnect (`self.WB_ClientConnect`))
  (if IsError
    (`/Game/GameBP/Blueprints/ClientConnect/UI/WB_Connect.SetError` _wb_clientconnect Message)
    (else
      (`/Game/GameBP/Blueprints/ClientConnect/UI/WB_Connect.SetStatus` _wb_clientconnect Message))))

(fn `GetNameFromPayload`
  (params (InfoResultPayload :type "PlayFabJsonObject Object Reference"))
  (returns (Username :type String))
  (locals (ResName :type String :default "N/A"))
  (`/Engine/EditorBlueprintResources/StandardMacros.IsValid` InfoResultPayload
    (:`Is Valid`
      (set `local.ResName` (`PlayFabJsonObject.GetStringField` (`PlayFabJsonObject.GetObjectField` InfoResultPayload "PlayerProfile") "DisplayName")))
    (:`Is Not Valid`
      _))
  (return (`local.ResName`)))

(fn `UserConstructionScript`)