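; Core Game Instance that handles the game's PlayFab backend connection.
; ConnectService logs in with a Google account, creating one if needed, and prints success or the error message.
; GetTitleData sends an Admin API title-data request for a given key and prints failures.
; Its success handler is empty, and the JSON object it builds with "SpecialCardsLimit" never feeds the request.
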(event `On Successful Connection`
  (params (result :type "ClientLoginResult Structure") (customData :type "Object Object Reference"))
  ;[1 1 1] Setup connection
  (`KismetSystemLibrary.PrintString` "Successful Login"))

(event `On Success: Get Title Data`
  (params (result :type "AdminGetTitleDataResult Structure") (customData :type "Object Object Reference")))

(event `Connect Service`
  ;[1 1 1] Setup connection
  (`PlayFabClientAPI.LoginWithGoogleAccount` (make `ClientLoginWithGoogleAccountRequest` true) (delegate `On Successful Connection`) (delegate `On Failed Connection`)))

(event `Get Title Data`
  (params (`Title Key` :type String))
  (bind _output_get (set `self.Json` (`PlayFabJsonObject.ConstructJsonObject`)))
  (`PlayFabJsonObject.SetStringField` _output_get `Title Key` "SpecialCardsLimit")
  (`PlayFabAdminAPI.GetTitleData` (make `AdminGetTitleDataRequest` `Title Key`) (delegate `On Success: Get Title Data`) (delegate `On Failure: Get Title Data`)))

(event `On Failed Connection`
  (params (error :type "PlayFabError Structure") (customData :type "Object Object Reference"))
  ;[1 1 1] Setup connection
  (`KismetSystemLibrary.PrintString` (`.ErrorMessage` (break `PlayFabError` error))))

(event `On Failure: Get Title Data`
  (params (error :type "PlayFabError Structure") (customData :type "Object Object Reference"))
  (`KismetSystemLibrary.PrintString` (`.ErrorMessage` (break `PlayFabError` error))))