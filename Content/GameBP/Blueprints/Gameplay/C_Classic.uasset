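; C_Classic is a locally controllable pawn whose first-person camera can jump to a seat position and back.
; On BeginPlay it activates FPCamera for the local player.
; MovetoSeatTransform saves the camera's current world transform, then applies the seat's location, pitch and yaw while keeping roll.
; BacktoOriginalSeat restores that transform if the camera location differs and the saved location is non-zero; both moves are instant, with interpolation marked TODO.
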(event `self.ReceiveBeginPlay`
  (if (`self.IsLocallyControlled`)
    (`ActorComponent.Activate` (`self.FP_Camera`) false)))

(event `Event Move to Seat Transform`
  (params (NewTransform :type "Transform Structure (by ref)"))
  (bind _fp_camera (`self.FP_Camera`))
  ;[1 0.5744 0.09237] TODO: Should interpolate (timeline)
  (bind _output_get (set `self.OriginalTransform` (`SceneComponent.K2_GetComponentToWorld` _fp_camera)))
  (`SceneComponent.K2_SetWorldTransform` _fp_camera (`KismetMathLibrary.MakeTransform` (.location NewTransform) (`KismetMathLibrary.MakeRotator` (.roll (.rotation _output_get)) (.pitch (.rotation NewTransform)) (.yaw (.rotation NewTransform)))) false false))

(event `Event Back to Original Seat`
  (bind _originaltransform (`self.OriginalTransform`))
  (bind _fp_camera (`self.FP_Camera`))
  (bind _location (.location _originaltransform))
  ;[1 0.5744 0.09237] TODO: Should interpolate --- Move back to original position
  (if (and (!= (.location (`SceneComponent.K2_GetComponentToWorld` _fp_camera)) _location) (!= _location (0.0 0.0 0.0)))
    (`SceneComponent.K2_SetWorldTransform` _fp_camera _originaltransform false false)))

(fn `UserConstructionScript`)