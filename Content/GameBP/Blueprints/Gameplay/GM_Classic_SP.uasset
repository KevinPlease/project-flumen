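; Single-player game mode for a pair-culling card game, with the local player at index 0 and AI objects filling the other seats.
; On play it creates and binds the AIs, then hands out decks once all connect.
; It confirms culls and card picks through CardMaster and relays them to player and AIs.
; GameState is told to start the roundtable, advance turns and mark finished or losing players.
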(event `self.ReceiveBeginPlay`
  ;[1 1 1] Begin Play
  (`parent.ReceiveBeginPlay`)
  (`KismetSystemLibrary.Delay` 2.0) ; delay to allow PC to init
  (bind _output_get (set `self.PlayerCount` (`/Game/GameBP/Blueprints/GI_Core.Matchmaking Size` (`self.GameInstanceRef`))))
  (`self.AddPlayerInQueue`)
  (`/Game/GameBP/Blueprints/Gameplay/Base/PC_Classic_Base.Event Matched` (`self.GetPlayerByIndex` 0) 0)
  (for _ (range 1 _output_get)
    (bind _playerindex (`self.AddPlayerInQueue`))
    (bind _ai (`self.CreateAI`))
    (`/Game/GameBP/Blueprints/Gameplay/Objects/O_AI.Event Matched` _ai _playerindex)))

(event `self.Event All Players Connected`
  (bind _gamestateref (`self.GameStateRef`))
  ;[1 1 1] Call player connected event to setup PC -> begin culling
  (`parent.Event All Players Connected`)
  (`/Game/GameBP/Blueprints/Gameplay/Base/PC_Classic_Base.Event Connected` (`self.GetPlayerByIndex` 0) (`/Game/GameBP/Blueprints/Gameplay/Objects/O_CardMaster.GetDecksForPlayer` (`self.CardMaster`) 0 (`/Game/GameBP/Blueprints/Gameplay/Base/GS_Classic_Base.PlayerNames` (`self.GameStateRef`))))
  (for _index (range 1 (`self.PlayerCount`))
    (`/Game/GameBP/Blueprints/Gameplay/Objects/O_AI.Event Connected` (`self.GetAiByIndex` _index) (`/Game/GameBP/Blueprints/Gameplay/Objects/O_CardMaster.GetDecksForPlayer` (`self.CardMaster`) _index (`/Game/GameBP/Blueprints/Gameplay/Base/GS_Classic_Base.PlayerNames` _gamestateref)) _gamestateref)))

(event `self.Event Player Culled Cards`
  (params (PlayerIndex :type Integer) (SelectedPair :type "/Game/GameData/Data/Gameplay/ST_Selection_CardPair Structure"))
  (bind (_gamefinished _playerlost) (`self.CheckVictoryConditions`))
  (`parent.Event Player Culled Cards` PlayerIndex SelectedPair)
  (if (not (`self.IsPlayer` PlayerIndex))
    (`/Game/GameBP/Blueprints/Gameplay/Base/PC_Classic_Base.Event Other Player Culled` (`self.GetPlayerByIndex` 0) PlayerIndex SelectedPair))
  (`|ExecutionSequence`
    (:`then_0`
      (switch `/Game/GameData/Data/Enums/E_GamePhases` (`/Game/GameBP/Blueprints/Gameplay/Base/GS_Classic_Base.GamePhase` (`self.GameStateRef`))
        (:`NewEnumerator0`
          ;[1 1 1] Check for remaining pairs -- if all players finished, tell GS to end the Culling phase
          (if (not (`/Game/GameBP/Blueprints/Gameplay/Objects/O_CardMaster.Has Remaining Pairs For Player` (`self.CardMaster`) PlayerIndex))
            (`self.SetPlayerReady` PlayerIndex)
            (if (`self.ArePlayersReady`)
              (`/Game/GameBP/Blueprints/Gameplay/Base/GS_Classic_Base.Event Begin RoundTable` (`self.GameStateRef`) (`self.FirstPlayerReady`) (`self.PlayerCount`)))))
        (:`NewEnumerator1`
          ;[1 1 1] Check if player who culled has remaining cards in hand
          (if (not (`/Game/GameBP/Blueprints/Gameplay/Objects/O_CardMaster.Has Remaining Cards For Player` (`self.CardMaster`) PlayerIndex)) :!label _label
            (`/Game/GameBP/Blueprints/Gameplay/Base/GS_Classic_Base.Event Player Finished` (`self.GameStateRef`) PlayerIndex false false 0.0))
          ;[1 1 1] Check for Finished Game
          (if _gamefinished
            (`/Game/GameBP/Blueprints/Gameplay/Base/GS_Classic_Base.Event Player Finished` (`self.GameStateRef`) _playerlost true false 0.0)))
        (:`NewEnumerator2`
          (goto _label))))
    (:`then_1`
      ;[1 1 1] Tell PC/AI that cull is confirmed and finished server-side
      (if (`self.IsPlayer` PlayerIndex)
        (`/Game/GameBP/Blueprints/Gameplay/Base/PC_Classic_Base.Event Cards Culled` (`self.GetPlayerByIndex` 0) true SelectedPair)
        (else
          (`/Game/GameBP/Blueprints/Gameplay/Objects/O_AI.Event Cards Culled` (`self.GetAiByIndex` PlayerIndex) true SelectedPair))))))

(event `self.Event Player Picked Card`
  (params (CardIndex :type Integer))
  (bind (_gamerule_id _gamerule_playercount _gamerule_cardrepetition _gamerule_timeperturn) (break `/Game/GameData/Data/Gameplay/ST_GameRule` (`self.GameRule`)))
  (bind _gamestateref (`self.GameStateRef`))
  (bind _gamestateref_2 (`self.GameStateRef`))
  (bind _gamestateref_3 (`self.GameStateRef`))
  (bind _activeplayerindex (`/Game/GameBP/Blueprints/Gameplay/Base/GS_Classic_Base.ActivePlayerIndex` _gamestateref_2))
  (bind _activeplayerindex_2 (`/Game/GameBP/Blueprints/Gameplay/Base/GS_Classic_Base.ActivePlayerIndex` _gamestateref))
  (bind _nextplayerindex (`/Game/GameBP/Blueprints/Gameplay/Base/GS_Classic_Base.NextPlayerIndex` (`self.GameStateRef`)))
  (bind _nextplayerindex_2 (`/Game/GameBP/Blueprints/Gameplay/Base/GS_Classic_Base.NextPlayerIndex` _gamestateref_2))
  (bind _nextplayerindex_3 (`/Game/GameBP/Blueprints/Gameplay/Base/GS_Classic_Base.NextPlayerIndex` _gamestateref_3))
  (bind _carddata (`/Game/GameBP/Blueprints/Gameplay/Objects/O_CardMaster.GetCardForPlayer` (`self.CardMaster`) (`/Game/GameBP/Blueprints/Gameplay/Base/GS_Classic_Base.NextPlayerIndex` _gamestateref) CardIndex))
  (`self.mIsPlayer` _activeplayerindex_2
    (:`Player`
      (`/Game/GameBP/Blueprints/Gameplay/Base/PC_Classic_Base.Event Card Added` (`self.GetPlayerByIndex` 0) _carddata))
    (:`AI`
      (`/Game/GameBP/Blueprints/Gameplay/Objects/O_AI.Event Card Added` (`self.GetAiByIndex` _activeplayerindex_2) _carddata)))
  (`/Game/GameBP/Blueprints/Gameplay/Objects/O_CardMaster.AddCardForPlayer` (`self.CardMaster`) _activeplayerindex_2 _carddata)
  (`self.mIsPlayer` _nextplayerindex
    (:`Player`
      (`/Game/GameBP/Blueprints/Gameplay/Base/PC_Classic_Base.Event Card Removed` (`self.GetPlayerByIndex` 0) CardIndex))
    (:`AI`
      (`/Game/GameBP/Blueprints/Gameplay/Objects/O_AI.Event Card Removed` (`self.GetAiByIndex` _nextplayerindex) CardIndex)))
  (`/Game/GameBP/Blueprints/Gameplay/Objects/O_CardMaster.RemoveCardForPlayer` (`self.CardMaster`) _nextplayerindex CardIndex)
  (`|ExecutionSequence`
    (:`then_0`
      (`self.mIsPlayer` _activeplayerindex
        (:`AI`
          (`/Game/GameBP/Blueprints/Gameplay/Base/PC_Classic_Base.Event Other PC Added Card` (`self.GetPlayerByIndex` 0) (make `/Game/GameData/Data/Gameplay/ST_AddedCard` _activeplayerindex (make `/Game/GameData/Data/Gameplay/ST_ClassicCard` -1))))))
    (:`then_1`
      (`self.mIsPlayer` _nextplayerindex_2
        (:`AI`
          (`/Game/GameBP/Blueprints/Gameplay/Base/PC_Classic_Base.Event Other PC Removed Card` (`self.GetPlayerByIndex` 0) (make `/Game/GameData/Data/Gameplay/ST_RemovedCard` _nextplayerindex_2 CardIndex)))))
    (:`then_2`
      ;[1 1 1] Check if the BeingPicked player has remaining cards in hand -- Next Turn
      (if (`/Game/GameBP/Blueprints/Gameplay/Objects/O_CardMaster.Has Remaining Cards For Player` (`self.CardMaster`) _nextplayerindex_3)
        (`/Game/GameBP/Blueprints/Gameplay/Base/GS_Classic_Base.Event Next Turn` _gamestateref_3 (`KismetMathLibrary.Conv_IntToDouble` _gamerule_timeperturn))
        (else
          (`/Game/GameBP/Blueprints/Gameplay/Base/GS_Classic_Base.Event Player Finished` _gamestateref_3 _nextplayerindex_3 false true (`KismetMathLibrary.Conv_IntToDouble` _gamerule_timeperturn)))))))

(fn `CreateAI`
  (returns (AI :type "/Game/GameBP/Blueprints/Gameplay/Objects/O_AI Object Reference"))
  (`|ExecutionSequence`
    (:`then_0`
      (bind _returnvalue (`|GenericCreateObject` "/Game/GameBP/Blueprints/Gameplay/Objects/O_AI.O_AI_C" self))
      (add `/Game/GameBP/Blueprints/Gameplay/Objects/O_AI.DispatchMatchedPlayer` _returnvalue (`|CreateDelegate` :!event `Event Matched Player`))
      (add `/Game/GameBP/Blueprints/Gameplay/Objects/O_AI.DispatchReadyToPlay` _returnvalue (`|CreateDelegate` :!event `Event Player Ready`))
      (add `/Game/GameBP/Blueprints/Gameplay/Objects/O_AI.DispatchCullingAttempt` _returnvalue (`|CreateDelegate` :!event `Event Player Culled Cards`))
      (add `/Game/GameBP/Blueprints/Gameplay/Objects/O_AI.DispatchPlayerPickedCard` _returnvalue (`|CreateDelegate` :!event `Event Player Picked Card`))
      (add `/Game/GameBP/Blueprints/Gameplay/Objects/O_AI.DispatchUpdateReadiness` _returnvalue (`|CreateDelegate` :!event `Event Update Player Readiness`)))
    (:`then_1`
      (`KismetArrayLibrary.Array_Add` (`self.ConnectedAIs`) _returnvalue)
      (return _returnvalue))))

(fn `GetAiByIndex`
  (params (AiIndex :type Integer))
  (returns (Ai :type "/Game/GameBP/Blueprints/Gameplay/Objects/O_AI Object Reference"))
  (return (`|GetArrayItem` (`self.ConnectedAIs`) (- AiIndex 1))))

(fn `IsPlayer`
  (params (PlayerIndex :type Integer))
  (returns (IsPlayer :type Boolean))
  (return (== PlayerIndex 0)))

(fn `UserConstructionScript`
  (`parent.UserConstructionScript`))