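; GS_Classic is the Classic mode game state that tracks the game phase and whose turn it is.
; Culling and round-table events set the phase, and starting either one fires a dispatcher to notify players; ending the culling only changes the phase.
; Round-table start and each turn end advance the active and next player indices, wrapping at the player count, then broadcast both.
; On authority, BeginPlay caches the GM_Classic game mode.
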(event `self.ReceiveBeginPlay`
  (if (`self.HasAuthority`)
    (bind _asgm_classic (cast `/Game/GameBP/Blueprints/Gameplay/GM_Classic` (`GameplayStatics.GetGameMode`)))
    (set `self.GameModeRef` _asgm_classic)))

(event `Event Begin Culling`
  ;[1 1 1] Call Players that the first phase has started
  (set `self.GamePhase` "NewEnumerator0")
  (`self.DispatchBeginCulling`))

(event `Event End The Culling`
  ;[1 1 1] Call Players that the first phase has started
  (set `self.GamePhase` "NewEnumerator2"))

(event `Event Begin RoundTable`
  (params (StartingPlayerIndex :type Integer) (PlayerCount :type Integer))
  ;[1 1 1] Update turn indices and dispatch the Begin Game event
  (set `self.Player Count` PlayerCount)
  (`self.UpdateNextPlayerIndex` StartingPlayerIndex)
  (set `self.GamePhase` "NewEnumerator1")
  (`self.DispatchBeginRoundtable` (`self.ActivePlayerIndex`) (`self.NextPlayerIndex`)))

(event `Event End Turn`
  ;[1 1 1] Call End Turn event for all clients
  (`self.UpdateNextPlayerIndex` (`self.NextPlayerIndex`))
  (`self.DispatchEndTurn` (`self.ActivePlayerIndex`) (`self.NextPlayerIndex`)))

(fn `UserConstructionScript`)