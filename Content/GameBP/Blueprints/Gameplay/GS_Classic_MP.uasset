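; GS_Classic_MP is the classic-mode multiplayer game state, handling turn and phase countdowns with separate server and client paths.
; BeginTurnTimer creates the turn timer on the authority, while clients start a phase counter.
; When the transition counter finishes, the authority fires the timer-ended event.
; Clients instead clear their counter timer, zero the UI phase counter and show the all-ready HUD message.
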(event `self.Event Finish Transition Counter`
  ;[1 1 1] Player updates own readiness state -- update server and clients
  (if (`self.HasAuthority`)
    (`self.Event Timer Ended`)
    (else
      (`KismetSystemLibrary.K2_ClearAndInvalidateTimerHandle` (`self.CounterTimer`))
      (bind _playercontrollerref (`self.GetPlayerControllerRef`))
      (`/Game/GameBP/Blueprints/Gameplay/Base/PC_Classic_Base.UI Update Phase Counter` _playercontrollerref 0)
      (`/Game/GameBP/Blueprints/Gameplay/UI/WB_HUD.Show All Ready Message` (`/Game/GameBP/Blueprints/Gameplay/Base/PC_Classic_Base.WB_HUD` _playercontrollerref)))))

(fn `BeginTurnTimer`
  (if (`self.HasAuthority`)
    (`self.Create Turn Timer` (`|CreateDelegate` :!event `Event Timer Ended`))
    (else
      (`self.Event Start Phase Counter`))))

(fn `UserConstructionScript`
  (`parent.UserConstructionScript`))