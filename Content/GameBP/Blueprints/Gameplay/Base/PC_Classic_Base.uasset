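; Base player controller for the classic multiplayer Donkey card game, where players cull pairs, pick from opponents' hands and the last one holding cards loses.
; Server RPCs forward matchmaking, readiness, culls, picks and reorders to the game mode.
; GameState dispatchers drive a local phase that controls input, HUD and seat camera moves.
; Touch taps select cards; long presses drag them through adjacent swaps, batching reorders until the next turn.
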(event `self.ReceiveBeginPlay`
  ;[1 1 1] Begin Play
  (if (`self.IsLocalPlayerController`)
    (`self.DisableInput` self)))

(event `ToServer: Matched`
  (params (DesiredMatchSize :type Integer) (PlayerIndex :type Integer) (PlayerServerInfo :type "/Game/GameData/Data/Player/ST_PlayerServerInfo Structure"))
  ;[1 1 1] Initial begin for PC --- Set index -> Send desired match size to GM
  (bind _asgm_classic_base (cast `/Game/GameBP/Blueprints/Gameplay/Base/GM_Classic_Base` (`GameplayStatics.GetGameMode`)))
  (bind _output_get (set `self.SV_GameModeRef` _asgm_classic_base))
  (`/Game/GameBP/Blueprints/Gameplay/Base/GM_Classic_Base.Event Matched Player` _output_get DesiredMatchSize PlayerIndex PlayerServerInfo))

(event `Event Matched`
  (params (PlayerIndex :type Integer))
  ;[1 1 1] Initial begin for PC --- Set index -> Send desired match size to GM
  (set `self.PlayerIndex` PlayerIndex)
  (bind _asgi_core (cast `/Game/GameBP/Blueprints/GI_Core` (`GameplayStatics.GetGameInstance`)))
  (bind _output_get (set `self.GameInstRef` _asgi_core))
  (bind _playerprofile (`/Game/GameBP/Blueprints/GI_Core.PlayerProfile` _output_get))
  (`self.ToServer: Matched` (`/Game/GameBP/Blueprints/GI_Core.Matchmaking Size` _output_get) (`self.PlayerIndex`) (make `/Game/GameData/Data/Player/ST_PlayerServerInfo` (`/Game/GameBP/Blueprints/ClientMenu/Objects/O_PlayerProfile.GetPlayfabId` _playerprofile) (`/Game/GameBP/Blueprints/ClientMenu/Objects/O_PlayerProfile.PlayerDisplayName` _playerprofile))))

(event `Event Connected`
  (params (DeckData :type "Array of /Game/GameData/Data/Gameplay/Wrappers/ST_CardList Structure"))
  (bind _gamestateref (`self.GameStateRef`))
  ;[1 1 1] Player connected with other player/s -- create HUD ...
  (bind _asc_classic (cast `/Game/GameBP/Blueprints/Gameplay/C_Classic` (`GameplayStatics.GetPlayerCharacter` 0)))
  (set `self.CharacterRef` _asc_classic)
  (bind _returnvalue (`|CreateWidget` "/Game/GameBP/Blueprints/Gameplay/UI/WB_HUD.WB_HUD_C" self))
  (bind _output_get (set `self.WB_HUD` _returnvalue))
  (`UserWidget.AddToViewport` _output_get 0)
  (bind _decks (`self.CreateDeckObj` DeckData))
  (`self.Create Board` _decks)
  (bind _asgs_classic_base (cast `/Game/GameBP/Blueprints/Gameplay/Base/GS_Classic_Base` (`GameplayStatics.GetGameState`)))
  (set `self.GameStateRef` _asgs_classic_base)
  (`|ExecutionSequence`
    (:`then_0`
      (add `/Game/GameBP/Blueprints/Gameplay/Base/GS_Classic_Base.DispatchBeginCulling` _gamestateref (`|CreateDelegate` :!event `Event On Begin Culling`))
      (add `/Game/GameBP/Blueprints/Gameplay/Base/GS_Classic_Base.DispatchEndCulling` _gamestateref (`|CreateDelegate` :!event `Event Finished Culling`))
      (add `/Game/GameBP/Blueprints/Gameplay/Base/GS_Classic_Base.DispatchEndCulling` _gamestateref (`|CreateDelegate` :!event `Event Finished Culling`))
      (add `/Game/GameBP/Blueprints/Gameplay/Base/GS_Classic_Base.DispatchNextTurn` _gamestateref (`|CreateDelegate` :!event `Event On Next Turn`))
      (add `/Game/GameBP/Blueprints/Gameplay/Base/GS_Classic_Base.DispatchTransitionPhase` _gamestateref (`|CreateDelegate` :!event `Event On Transition Phase`))
      (add `/Game/GameBP/Blueprints/Gameplay/Base/GS_Classic_Base.DispatchEmptyDeckForPlayer` _gamestateref (`|CreateDelegate` :!event `Event On Empty Deck`))
      (add `/Game/GameBP/Blueprints/Gameplay/Base/GS_Classic_Base.DispatchGameOver` _gamestateref (`|CreateDelegate` :!event `Event Game Over`)))
    (:`then_1`
      ;[1 1 1] Player has connected successfully and is ready to start game
      (`self.To Server: Ready To Play` (`self.PlayerIndex`)) ; Player setup finished
    )))

(event `To Server: Ready To Play`
  (params (PlayerIndex :type Integer))
  ;[1 1 1] Player has connected successfully and is ready to start game
  (`/Game/GameBP/Blueprints/Gameplay/Base/GM_Classic_Base.Event Player Ready` (`self.SV_GameModeRef`) PlayerIndex))

(event `Event Clicked Card`
  (params (ClickedCardActor :type "/Game/GameBP/Blueprints/Gameplay/Actors/BP_Card Object Reference"))
  (bind _carddata_label (break `/Game/GameData/Data/Gameplay/ST_ClassicCard` (`/Game/GameBP/Blueprints/Gameplay/Actors/BP_Card.CardData` ClickedCardActor)))
  (bind _indexinhand (`/Game/GameBP/Blueprints/Gameplay/Actors/BP_Card.IndexInHand` ClickedCardActor))
  ;[1 1 1] Input: Single Click on Card
  (switch `/Game/GameData/Data/Enums/E_PlayerPhases` (`self.ActivePhase`)
    (:`NewEnumerator4`
      (if (not (`/Game/GameBP/Blueprints/Gameplay/Actors/BP_Card.IsSelected` ClickedCardActor)) :!label _label
        (`/Game/GameBP/Blueprints/Gameplay/Actors/BP_Card.Select` ClickedCardActor)
        (`/Engine/EditorBlueprintResources/StandardMacros.CompareInt` (`self.FirstSelectedCardLabel`) -1 ; Check if 2 cards have been selected
          (:`>`
            (set `self.SecondCardIndex` _indexinhand)
            (`self.DisableInput` self) ; no quick-culling
            (`self.To Server: Culled Cards` (`self.PlayerIndex`) (make `/Game/GameData/Data/Gameplay/ST_Selection_CardPair` 0 0 (`self.FirstCardIndex`) (`self.SecondCardIndex`)))
            (`self.ResetSelection`))
          (:`==`
            (set `self.FirstSelectedCardLabel` _carddata_label)
            (set `self.FirstCardIndex` _indexinhand)))
        (else
          (`/Game/GameBP/Blueprints/Gameplay/Actors/BP_Card.Deselect` ClickedCardActor)
          (`self.ResetSelection`))))
    (:`NewEnumerator0`
      (goto _label))
    (:`NewEnumerator1`
      (`self.DisableInput` self) ; no quick-picking
      (`self.To Server: Picked Card From Player` _indexinhand))
    (:`NewEnumerator6`
      (goto _label))))

(event `Event Player Forfeits`
  ;[1 1 1] Player forfeits OR safe leaves after finishing
  (`/Game/GameBP/Blueprints/GI_Core.LoadClientMap` (`self.GameInstRef`)))

(event `Event Safe Leave`
  (bind _gamestateref (`self.GameStateRef`))
  ;[1 1 1] Player forfeits OR safe leaves after finishing
  (`/Game/GameBP/Blueprints/Gameplay/UI/WB_HUD.ShowGameResults` (`self.WB_HUD`) (`/Game/GameBP/Blueprints/Gameplay/Base/GS_Classic_Base.GetGameResults` _gamestateref) (`/Game/GameBP/Blueprints/Gameplay/Base/GS_Classic_Base.Player Count` _gamestateref)))

(event `InputTouch`
  (params (Location :type "Vector Structure") (FingerIndex :type "ETouchIndex Enum"))
  ;[1 1 1] Handle touch input
  (:`Pressed`
    (bind _asbp_card (cast `/Game/GameBP/Blueprints/Gameplay/Actors/BP_Card` (`.HitActor` (`GameplayStatics.BreakHitResult` (`self.GetHitResultUnderFingerForObjects` "Touch1" (`|MakeArray` "ObjectTypeQuery1" :!type "EObjectTypeQuery Enum")))))
      (:`then`
        (`self.InputPress` :!label _label_2
          (:`LongPress`
            (if (`|EnumInequality` (`self.ActivePhase`) "NewEnumerator4")
              (`self.StartCardHolding` null)))
          (:`SinglePress`
            (`self.IsValidSelection` _asbp_card
              (:`Valid`
                (`self.Event Clicked Card` _asbp_card))))))
      (:`CastFailed`
        ;;[1 1 1] Selection on empty area
        (`self.Event Reset Card Selection`)
        (`/Game/GameBP/Blueprints/Gameplay/UI/WB_HUD.SafeHideInGameMenu` (`self.WB_HUD`)))))
  (:`Released`
    (`|ExecutionSequence`
      (:`then_0`
        (if (not (`self.IsHoldingCard`))
          (goto _label_2 :!via `Released`)))
      (:`then_1`
        (if (`self.IsHoldingCard`)
          (`self.StopCardHolding`)))))
  (:`Moved`
    (if (`self.IsHoldingCard`)
      (`/Engine/EditorBlueprintResources/StandardMacros.DoOnce` false :!label _label_3
        (:`Completed`
          (bind _asbp_card_2 (`self.CheckMovingInputBounds`)
            (:`Overlapped Seeking Card`
              (`self.Event Card Seeking Position` _asbp_card_2))
            (:`No Card But Within Deck Bounds`
              (`self.InternalResetMovingInput` :!label _label_4))
            (:`Out Of Deck Bounds`
              (goto _label_4))))))))

(event `InternalResetMovingInput`
  ;[1 1 1] Handle touch input
  (goto _label_3 :!via `Reset`))

(event `Event Reset Card Seeking`
  ;[1 1 1] Handle touch input
  (`/Engine/EditorBlueprintResources/StandardMacros.IsValid` (`self.CurSeekingCard`)
    (:`Is Valid`
      (set `self.CurSeekingCard` null)
      (goto _label_3 :!via `Reset`))
    (:`Is Not Valid`
      (goto _label_3 :!via `Reset`))))

(event `Event Prepare For Next Phase`
  ;[1 1 1] Reset all selections, card seeking
  (if (`self.IsHoldingCard`)
    (`self.StopCardHolding`))
  (`self.Event Reset Card Selection`)
  (`self.Event Reset Card Seeking`)
  (`self.SendRepositioningRequest`))

(event `Event Reset Card Selection`
  (bind _asbp_card (`/Game/GameBP/Blueprints/Gameplay/Actors/BP_CardDeck.Get Card As Actor` (`self.PlayerDeck`) (`self.FirstCardIndex`)))
  ;[1 1 1] Reset all selections, card seeking
  (`/Engine/EditorBlueprintResources/StandardMacros.IsValid` _asbp_card
    (:`Is Valid`
      (if (`/Game/GameBP/Blueprints/Gameplay/Actors/BP_Card.IsSelected` _asbp_card)
        (`/Game/GameBP/Blueprints/Gameplay/Actors/BP_Card.Deselect` _asbp_card)
        (`self.ResetSelection`)))))

(event `ToServer: Event Update Readiness`
  (params (IsReadyToSkip :type Boolean) (PlayerIndex :type Integer))
  ;[1 1 1] Mark self as ready to skip transition
  (`/Game/GameBP/Blueprints/Gameplay/Base/GM_Classic_Base.Event Update Player Readiness` (`self.SV_GameModeRef`) PlayerIndex IsReadyToSkip))

(event `Event On Transition Phase`
  ;[1 1 1] Next Turn
  (if (`self.IsPlaying`)
    (set `self.ActivePhase` "NewEnumerator6")
    (`self.UI Update Player Phase`)
    (`/Game/GameBP/Blueprints/Gameplay/C_Classic.Event Back to Original Seat` (`self.CharacterRef`))))

(event `Event Ready To Skip Transition`
  ;[1 1 1] Mark self as ready to skip transition
  (`self.DisableInput` self)
  (`self.ToServer: Event Update Readiness` true (`self.PlayerIndex`)))

(event `Event On Next Turn`
  (params (PlayerIndex :type Integer) (NextPlayerIndex :type Integer) (FirstTime :type Boolean))
  ;[1 1 1] Next Turn
  (if (`self.IsPlaying`)
    (if FirstTime
      (`self.FirstRoundUpdate` PlayerIndex)
      (`KismetSystemLibrary.Delay` 1.0))
    (if (`|EnumEquality` (`self.ActivePhase`) "NewEnumerator1")
      (`/Game/GameBP/Blueprints/Gameplay/C_Classic.Event Back to Original Seat` (`self.CharacterRef`))
      (`self.UpdatePostAnimInput` false))
    (`self.UpdatePhase` PlayerIndex NextPlayerIndex)
    (`self.UI Update Player Phase`)
    (`self.Event Prepare For Next Phase`)
    (switch `/Game/GameData/Data/Enums/E_PlayerPhases` (`self.ActivePhase`)
      (:`NewEnumerator1`
        (`/Game/GameBP/Blueprints/Gameplay/C_Classic.Event Move to Seat Transform` (`self.CharacterRef`) (`/Game/GameBP/Blueprints/Gameplay/Actors/BP_GameBoard.Get Seat Transform For Player` (`self.GameBoard`) NextPlayerIndex))
        (`self.UpdatePostAnimInput` true))
      (:`NewEnumerator7`
        (`self.Event Force Game Over`)))))

(event `Event Card Removed`
  (params (CardIndex :type Integer))
  ;[1 1 1] Card was removed/added - notify own Deck
  (`/Game/GameBP/Blueprints/Gameplay/Actors/BP_CardDeck.Event Removed Card` (`self.PlayerDeck`) CardIndex)
  (`self.ResetSelection`) ; Case when 1 card was selected during culling process,\nbut other player picked it during his/her Picking phase
)

(event `Event On Empty Deck`
  (params (PlayerIndex :type Integer))
  ;[1 1 1] Player emptied Deck -- go into spectating mode
  (if (== PlayerIndex (`self.PlayerIndex`))
    (set `self.ActivePhase` "NewEnumerator3")
    (`self.DisableInput` self)
    (`self.UI Update Player Phase`)
    (`/Game/GameBP/Blueprints/Gameplay/C_Classic.Event Back to Original Seat` (`self.CharacterRef`))
    (else
      ;[1 0.5744 0.09237] TODO: Might update GameBoard to show something in the location of the player-who-'won''s deck
      (`KismetSystemLibrary.PrintString` "Another player won..."))))

(event `Event Card Seeking Position`
  (params (InCard :type "/Game/GameBP/Blueprints/Gameplay/Actors/BP_Card Object Reference"))
  ;[1 1 1] A picked up card is seeking for a new position -- Shift cards left/right to make room while Picked up card traverses Deck
  (bind _output_get (set `self.CurSeekingCard` InCard))
  (`/Game/GameBP/Blueprints/Gameplay/Actors/BP_CardDeck.SwapCards` (`self.PlayerDeck`) (`self.HoldingCard`) _output_get)
  (`self.InternalResetMovingInput`))

(event `Event Card Added`
  (params (CardData :type "/Game/GameData/Data/Gameplay/ST_ClassicCard Structure"))
  ;[1 1 1] Card was removed/added - notify own Deck
  (`/Game/GameBP/Blueprints/Gameplay/Actors/BP_CardDeck.Event Added Card` (`self.PlayerDeck`) CardData))

(event `Event Other PC Removed Card`
  (params (RemovedCardDeal :type "/Game/GameData/Data/Gameplay/ST_RemovedCard Structure"))
  ;[1 1 1] Other PC made changes to his/her deck -- update actors
  (`/Game/GameBP/Blueprints/Gameplay/Actors/BP_GameBoard.Event Card Removed By Player` (`self.GameBoard`) RemovedCardDeal))

(event `Event Other PC Added Card`
  (params (ST_AddedCard :type "/Game/GameData/Data/Gameplay/ST_AddedCard Structure (by ref)"))
  ;[1 1 1] Other PC made changes to his/her deck -- update actors
  (`/Game/GameBP/Blueprints/Gameplay/Actors/BP_GameBoard.Event Card Added By Player` (`self.GameBoard`) ST_AddedCard))

(event `ToServer: CardsRepositioned`
  (params (PlayerIndex :type Integer) (CardsRepositioned :type "Array of /Game/GameData/Data/Gameplay/ST_Selection_CardPair Structure"))
  ;[1 1 1] Cards repositioned in deck -- notify GM to update indices
  (`/Game/GameBP/Blueprints/Gameplay/Base/GM_Classic_Base.Event Player Repositioned Cards` (`self.SV_GameModeRef`) PlayerIndex CardsRepositioned))

(event `Event Game Over`
  (params (PlayerLost :type Integer))
  (bind _gamestateref (`self.GameStateRef`))
  ;[1 1 1] A player has lost -- check if self -- Game Over
  (if (== PlayerLost (`self.PlayerIndex`))
    (`self.DisableInput` self)
    (`/Game/GameBP/Blueprints/Gameplay/C_Classic.Event Back to Original Seat` (`self.CharacterRef`))
    (`KismetSystemLibrary.Delay` 1.0)
    (`/Game/GameBP/Blueprints/Gameplay/Actors/BP_CardDeck.Event Play Donkey In Hand Fx` (`self.PlayerDeck`) true) ; index 0 since is last card
    (`KismetSystemLibrary.Delay` 1.5))
  (`/Game/GameBP/Blueprints/Gameplay/UI/WB_HUD.ShowGameResults` (`self.WB_HUD`) (`/Game/GameBP/Blueprints/Gameplay/Base/GS_Classic_Base.GetGameResults` _gamestateref) (`/Game/GameBP/Blueprints/Gameplay/Base/GS_Classic_Base.Player Count` _gamestateref)))

(event `To Server: Picked Card From Player`
  (params (PickedCardIndex :type Integer))
  ;[1 1 1] Tell GM about the picked card index
  (`/Game/GameBP/Blueprints/Gameplay/Base/GM_Classic_Base.Event Player Picked Card` (`self.SV_GameModeRef`) PickedCardIndex))

(event `Event Return to Main Menu`
  (bind _gameinstref (`self.GameInstRef`))
  ;[1 1 1] Back to Main Menu with the game finished results
  (set `/Game/GameBP/Blueprints/GI_Core.GameResult` (`/Game/GameBP/Blueprints/Gameplay/Base/GS_Classic_Base.GetResultForPlayer` (`self.GameStateRef`) (`self.PlayerIndex`)) _gameinstref)
  (`/Game/GameBP/Blueprints/GI_Core.LoadClientMap` _gameinstref))

(event `Event Force Game Over`
  ;[1 1 1] Force the last player to finish -- autoremove last pair from hand -- show game over UI
  (`self.To Server: Culled Cards` (`self.PlayerIndex`) (`/Game/GameBP/Blueprints/Gameplay/Objects/O_CardDeck.GetLastCardPair` (`/Game/GameBP/Blueprints/Gameplay/Actors/BP_CardDeck.CardDeck` (`self.PlayerDeck`)))))

(event `Event On Begin Culling`
  ;[1 1 1] Begin Phase
  (set `self.ActivePhase` "NewEnumerator4")
  (`self.UI Update Player Phase`))

(event `To Server: Culled Cards`
  (params (PlayerIndex :type Integer) (CardPair :type "/Game/GameData/Data/Gameplay/ST_Selection_CardPair Structure"))
  ;[1 1 1] Tell server cards of Culling attempt
  (`/Game/GameBP/Blueprints/Gameplay/Base/GM_Classic_Base.Event Player Culled Cards` (`self.SV_GameModeRef`) PlayerIndex CardPair))

(event `Event Cards Culled`
  (params (IsValid :type Boolean) (CardPair :type "/Game/GameData/Data/Gameplay/ST_Selection_CardPair Structure"))
  (bind (_firstlabel _secondlabel _firstposition _secondposition) (break `/Game/GameData/Data/Gameplay/ST_Selection_CardPair` CardPair))
  (bind _playerdeck (`self.PlayerDeck`))
  ;[1 1 1] Tell server cards of Culling attempt
  (if IsValid
    (`KismetSystemLibrary.Delay` 0.2) ; to allow animation to finish
    (`/Game/GameBP/Blueprints/Gameplay/Actors/BP_CardDeck.Event Cull Cards` _playerdeck (make `/Game/GameData/Data/Gameplay/ST_Selection_CardPair` 0 0 _firstposition _secondposition))
    (`KismetSystemLibrary.Delay` 1.0) ; to allow animation to finish
    (else
      (`self.PlayShakeAndVibrate`)
      (`KismetSystemLibrary.Delay` 0.2) ; to allow animation to finish
      (`/Game/GameBP/Blueprints/Gameplay/Actors/BP_CardDeck.Event Bad Cull Attempt` _playerdeck (make `/Game/GameData/Data/Gameplay/ST_Selection_CardPair` 0 0 _firstposition _secondposition))))
  (`self.UpdatePlayerInputPerPhase`))

(event `Event Other Player Culled`
  (params (OtherPlayerIndex :type Integer) (CardPair :type "/Game/GameData/Data/Gameplay/ST_Selection_CardPair Structure"))
  ;[1 1 1] Other player has culled cards -- update GameBoard
  (`/Game/GameBP/Blueprints/Gameplay/Actors/BP_GameBoard.Event Pair Removed By Player` (`self.GameBoard`) OtherPlayerIndex CardPair))

(event `Event Finished Culling`
  ;[1 1 1] Server says Culling phase is over - disable input etc...
  (`self.DisableInput` self)
  (set `self.ActivePhase` "NewEnumerator0")
  (`self.UI Update Player Phase`))

(fn `Create Board`
  (params (Decks :type "Array of /Game/GameBP/Blueprints/Gameplay/Objects/O_CardDeck Object Reference"))
  (bind _playerprofile (`/Game/GameBP/Blueprints/GI_Core.PlayerProfile` (`self.GameInstRef`)))
  (bind _returnvalue (`|SpawnActorFromClass` "/Game/GameBP/Blueprints/Gameplay/Actors/BP_GameBoard.BP_GameBoard_C" (`self.GetSpawnLocation`) "DontSpawnIfColliding" "OverrideRootScale" self (`/Game/GameBP/Blueprints/ClientMenu/Objects/O_PlayerProfile.GetBoardTheme` _playerprofile) (`/Game/GameBP/Blueprints/ClientMenu/Objects/O_PlayerProfile.GetCardTheme` _playerprofile) null))
  (bind _output_get (set `self.GameBoard` _returnvalue))
  (`/Game/GameBP/Blueprints/Gameplay/Actors/BP_GameBoard.Event Create With Data` _output_get Decks (`self.PlayerIndex`))
  (set `self.PlayerDeck` (`/Game/GameBP/Blueprints/Gameplay/Actors/BP_GameBoard.GetDeckActorForPlayer` _output_get (`self.PlayerIndex`))))

(fn `CreateDeckObj`
  (params (DeckData :type "Array of /Game/GameData/Data/Gameplay/Wrappers/ST_CardList Structure"))
  (returns (Decks :type "Array of /Game/GameBP/Blueprints/Gameplay/Objects/O_CardDeck Object Reference"))
  (locals (CurCardDeck :type "/Game/GameBP/Blueprints/Gameplay/Objects/O_CardDeck Object Reference") (DeckObjs :type "Array of /Game/GameBP/Blueprints/Gameplay/Objects/O_CardDeck Object Reference"))
  (bind _curcarddeck (`local.CurCardDeck`))
  (for (_array_element _array_index) DeckData
    (if (== _array_index (`self.PlayerIndex`))
      (bind _returnvalue (`|GenericCreateObject` "/Game/GameBP/Blueprints/Gameplay/Objects/O_PlayerDeck.O_PlayerDeck_C" self))
      (set `local.CurCardDeck` _returnvalue)
      (else
        (bind _returnvalue_2 (`|GenericCreateObject` "/Game/GameBP/Blueprints/Gameplay/Objects/O_EnemyDeck.O_EnemyDeck_C" self))
        (set `local.CurCardDeck` _returnvalue_2)))
    (bind (_cards _playername) (break `/Game/GameData/Data/Gameplay/Wrappers/ST_CardList` _array_element))
    (`/Game/GameBP/Blueprints/Gameplay/Objects/O_CardDeck.Create` _curcarddeck _cards _playername)
    (`KismetArrayLibrary.Array_Add` (`local.DeckObjs`) _curcarddeck))
  (return (`local.DeckObjs`)))

(fn `FirstRoundUpdate`
  (params (ActivePlayerIndex :type Integer))
  (`/Game/GameBP/Blueprints/Gameplay/UI/WB_HUD.Event Show General Delayed Message` (`self.WB_HUD`) (`|FormatText` "{text1} ishte shumë i shpejt'!!" (`KismetTextLibrary.Conv_StringToText` (`/Game/GameBP/Blueprints/Gameplay/Base/GS_Classic_Base.GetPlayerName` (`self.GameStateRef`) ActivePlayerIndex))) 3.0))

(fn `GetSpawnLocation`
  (returns (SpawnTransform :type "Transform Structure"))
  (locals (YawMultiplier :type "Float (double-precision)" :default 0.0))
  (switch `int` (`self.PlayerIndex`)
    (:`0`
      (set `local.YawMultiplier` 0.0))
    (:`1`
      (set `local.YawMultiplier` 90.0))
    (:`2`
      (set `local.YawMultiplier` -90.0))
    (:`3`
      (set `local.YawMultiplier` -180.0)))
  (return (`KismetMathLibrary.MakeTransform` (0.0 0.0 144.0) (`KismetMathLibrary.MakeRotator` 0.0 0.0 (`local.YawMultiplier`)))))

(fn `IsHoldingCard`
  (returns (IsHolding :type Boolean))
  (return (`KismetSystemLibrary.IsValid` (`self.HoldingCard`))))

(fn `IsPlaying`
  (returns (InGameplay :type Boolean))
  (bind _activephase (`self.ActivePhase`))
  (return (and (`|EnumInequality` _activephase "NewEnumerator3") (`|EnumInequality` _activephase "NewEnumerator7"))))

(fn `IsValidSeekingCardPos`
  (params (Card :type "/Game/GameBP/Blueprints/Gameplay/Actors/BP_Card Object Reference"))
  (returns (ReturnValue :type Boolean))
  (bind _holdingcard (`self.HoldingCard`))
  (if (`KismetSystemLibrary.IsValid` _holdingcard)
    (return (!= (`/Game/GameBP/Blueprints/Gameplay/Actors/BP_Card.IndexInHand` Card) (+ (`/Game/GameBP/Blueprints/Gameplay/Actors/BP_Card.IndexInHand` _holdingcard) 1)))
    (else
      (return false))))

(fn `PlayShakeAndVibrate`
  (bind (_optionsdata_mastervolume _optionsdata_musicvolume _optionsdata_sfxvolume _optionsdata_uivolume _optionsdata_vibrations) (break `/Game/GameData/Data/Player/ST_Options` (`/Game/GameBP/Blueprints/ClientMenu/Objects/O_PlayerProfile.OptionsData` (`/Game/GameBP/Blueprints/GI_Core.PlayerProfile` (`self.GameInstRef`)))))
  (`GameplayStatics.PlayWorldCameraShake` "/Game/GameBP/Blueprints/Gameplay/Effects/VFX/BP_CameraShake.BP_CameraShake_C" (`self.K2_GetActorLocation` (`self.CharacterRef`)) 0.0 1500.0)
  (if _optionsdata_vibrations
    (`self.K2_ClientPlayForceFeedback` self "/Game/GameBP/Blueprints/Gameplay/Effects/VFX/FF_Rumble.FF_Rumble" "None" false false false)))

(fn `ResetSelection`
  (set `self.FirstSelectedCardLabel` -1)
  (set `self.FirstCardIndex` -1)
  (set `self.SecondCardIndex` -1))

(fn `SendRepositioningRequest`
  (bind _cardsrepositioned (`self.CardsRepositioned`))
  (if (> (`KismetArrayLibrary.Array_Length` _cardsrepositioned) 0)
    (`self.ToServer: CardsRepositioned` (`self.PlayerIndex`) _cardsrepositioned)
    (`KismetArrayLibrary.Array_Clear` (`self.CardsRepositioned`))))

(fn `StartCardHolding`
  (params (CardActor :type "/Game/GameBP/Blueprints/Gameplay/Actors/BP_Card Object Reference"))
  (`/Game/GameBP/Blueprints/Gameplay/Actors/BP_Card.TogglePickupMode` CardActor true)
  (bind _output_get (set `self.HoldingCard` CardActor))
  (set `self.CurHoldingCardOrigIndex` (`/Game/GameBP/Blueprints/Gameplay/Actors/BP_Card.IndexInHand` _output_get)))

(fn `StopCardHolding`
  (`/Game/GameBP/Blueprints/Gameplay/Actors/BP_Card.TogglePickupMode` (`self.HoldingCard`) false)
  (if (`KismetSystemLibrary.IsValid` (`self.CurSeekingCard`))
    (`KismetArrayLibrary.Array_Add` (`self.CardsRepositioned`) (make `/Game/GameData/Data/Gameplay/ST_Selection_CardPair` 0 0 (`self.CurHoldingCardOrigIndex`) (`/Game/GameBP/Blueprints/Gameplay/Actors/BP_Card.IndexInHand` (`self.HoldingCard`))))
    (else
      (`/Game/GameBP/Blueprints/Gameplay/Actors/BP_CardDeck.Reset Location for Card` (`self.PlayerDeck`) (`self.HoldingCard`))))
  (set `self.HoldingCard` null)
  (set `self.CurSeekingCard` null))

(fn `UI Update Phase Counter`
  (params (Counter :type Integer))
  (`/Game/GameBP/Blueprints/Gameplay/UI/WB_HUD.SetCounter` (`self.WB_HUD`) Counter))

(fn `UI Update Player Phase`
  (bind _wb_hud (`self.WB_HUD`))
  (bind _activephase (`self.ActivePhase`))
  (`/Game/GameBP/Blueprints/Gameplay/UI/WB_HUD.SetPlayerPhaseText` _wb_hud _activephase)
  (`self.UpdatePlayerInputPerPhase`)
  (switch `/Game/GameData/Data/Enums/E_PlayerPhases` _activephase
    (:`NewEnumerator6`
      (`/Game/GameBP/Blueprints/Gameplay/UI/WB_HUD.ResetReadyButton` _wb_hud))))

(fn `UpdateHoldingCard`)

(fn `UpdatePhase`
  (params (ActivePlayerIndex :type Integer) (NextPlayerIndex :type Integer))
  (bind _playerindex (`self.PlayerIndex`))
  (if (== ActivePlayerIndex _playerindex)
    (if (`/Game/GameBP/Blueprints/Gameplay/Base/GS_Classic_Base.IsLastPlayer` (`self.GameStateRef`) (`self.PlayerIndex`))
      (set `self.ActivePhase` "NewEnumerator7")
      (else
        (set `self.ActivePhase` "NewEnumerator1")))
    (elif (== NextPlayerIndex _playerindex)
      (set `self.ActivePhase` "NewEnumerator2")
      (else
        (set `self.ActivePhase` "NewEnumerator0")))))

(fn `UpdatePlayerInputPerPhase`
  (switch `/Game/GameData/Data/Enums/E_PlayerPhases` (`self.ActivePhase`)
    (:`NewEnumerator4`
      (`self.EnableInput` self :!label _label))
    (:`NewEnumerator0`
      (goto _label))
    (:`NewEnumerator1`
      (goto _label))
    (:`NewEnumerator2`
      (`self.DisableInput` self :!label _label_2))
    (:`NewEnumerator3`
      (goto _label_2))
    (:`NewEnumerator6`
      (goto _label))))

(fn `UserConstructionScript`)