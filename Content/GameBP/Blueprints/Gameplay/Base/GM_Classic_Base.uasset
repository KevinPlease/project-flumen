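; Base game mode for a classic Donkey card game, running player matching, pair culling and card picks from the next player.
; Once all players connect, it loads a rule row by player count and has an O_CardMaster object set up the decks.
; When all report ready, the game state begins culling.
; It validates culls by matching labels, relays picks and repositions to CardMaster, and currently resolves every player to controller 0.
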(event `self.ReceiveBeginPlay`
  ;[1 1 1] BeginPlay - Get references
  (bind _asgs_classic_base (cast `/Game/GameBP/Blueprints/Gameplay/Base/GS_Classic_Base` (`GameplayStatics.GetGameState`)))
  (set `self.GameStateRef` _asgs_classic_base)
  (bind _asgi_core (cast `/Game/GameBP/Blueprints/GI_Core` (`GameplayStatics.GetGameInstance`)))
  (set `self.GameInstanceRef` _asgi_core)
  (bind _returnvalue (`|GenericCreateObject` "/Game/GameBP/Blueprints/Gameplay/Objects/O_CardMaster.O_CardMaster_C" self))
  (set `self.CardMaster` _returnvalue))

(event `Event Matched Player`
  (params (DesiredMatchSize :type Integer) (PlayerIndex :type Integer) (PlayerServerInfo :type "/Game/GameData/Data/Player/ST_PlayerServerInfo Structure"))
  ;[1 1 1] Event matched player -- check if first and if all players are connected
  (if (== PlayerIndex 0)
    (set `self.PlayerCount` DesiredMatchSize))
  (`self.UpdatePlayerConnected` PlayerIndex PlayerServerInfo_PlayerName_4_82062F2C46B696FF488639B7BB118ADD)
  (if (`self.AreAllPlayersConnected`)
    (`self.Event All Players Connected`)
    (else
      (`KismetSystemLibrary.PrintString` "Not enough players connected"))))

(event `Event All Players Connected`
  (bind (_gamerule_id _gamerule_playercount _gamerule_cardrepetition) (break `/Game/GameData/Data/Gameplay/ST_GameRule` (`self.GameRule`)))
  ;[1 1 1] Load game rules, setup cards based on rules
  (`self.LoadGameRules` (`self.PlayerCount`))
  (`/Game/GameBP/Blueprints/Gameplay/Objects/O_CardMaster.Setup Cards For Players` (`self.CardMaster`) _gamerule_playercount _gamerule_cardrepetition))

(event `Event Player Ready`
  (params (PlayerIndex :type Integer))
  (bind _gamestateref (`self.GameStateRef`))
  (bind (_gamerule_id _gamerule_playercount _gamerule_cardrepetition _gamerule_timeperturn) (break `/Game/GameData/Data/Gameplay/ST_GameRule` (`self.GameRule`)))
  ;[1 1 1] BEGIN gameplay once all players are ready i.e: decks created etc.
  (`self.SetPlayerReady` PlayerIndex)
  (if (`self.ArePlayersReady`)
    (for _index (range (`self.PlayerCount`))
      (`self.ResetPlayerReady` _index)
      (`/Game/GameBP/Blueprints/Gameplay/Base/GS_Classic_Base.Event Update Player Name` _gamestateref (`/Game/GameBP/Blueprints/Gameplay/Base/GS_Classic_Base.PlayerNames` _gamestateref)))
    (`/Game/GameBP/Blueprints/Gameplay/Base/GS_Classic_Base.Event Begin Culling` (`self.GameStateRef`) _gamerule_timeperturn)))

(event `Event Player Repositioned Cards`
  (params (PlayerIndex :type Integer) (CardsRepositioned :type "Array of /Game/GameData/Data/Gameplay/ST_Selection_CardPair Structure"))
  ;[1 1 1] Player made card reposition request -- update CardMaster
  (`self.UpdateCardRepositioning` PlayerIndex CardsRepositioned))

(event `Event Player Picked Card`
  (params (CardIndex :type Integer))
  (bind _gamestateref (`self.GameStateRef`))
  (bind _activeplayerindex (`/Game/GameBP/Blueprints/Gameplay/Base/GS_Classic_Base.ActivePlayerIndex` _gamestateref))
  (bind _carddata (`/Game/GameBP/Blueprints/Gameplay/Objects/O_CardMaster.GetCardForPlayer` (`self.CardMaster`) (`/Game/GameBP/Blueprints/Gameplay/Base/GS_Classic_Base.NextPlayerIndex` _gamestateref) CardIndex))
  ;[1 1 1] Player picked a card from the next player -- End turn
  (`/Game/GameBP/Blueprints/Gameplay/Base/PC_Classic_Base.Event Card Added` (`self.GetPlayerByIndex` _activeplayerindex) _carddata)
  (`/Game/GameBP/Blueprints/Gameplay/Objects/O_CardMaster.AddCardForPlayer` (`self.CardMaster`) _activeplayerindex _carddata))

(event `Event Update Player Readiness`
  (params (PlayerIndex :type Integer) (IsReadyToSkip :type Boolean))
  ;[1 1 1] Update readiness state for player
  (`/Game/GameBP/Blueprints/Gameplay/Base/GS_Classic_Base.Event Player Updated Readiness` (`self.GameStateRef`) PlayerIndex IsReadyToSkip))

(event `Event Player Culled Cards`
  (params (PlayerIndex :type Integer) (SelectedPair :type "/Game/GameData/Data/Gameplay/ST_Selection_CardPair Structure"))
  ;[1 1 1] Player has selected two cards to cull
  (if (`self.IsValidCullAttempt` PlayerIndex SelectedPair)
    (`/Game/GameBP/Blueprints/Gameplay/Objects/O_CardMaster.RemoveCardPair` (`self.CardMaster`) PlayerIndex SelectedPair)
    (else
      (`/Game/GameBP/Blueprints/Gameplay/Base/PC_Classic_Base.Event Cards Culled` (`self.GetPlayerByIndex` PlayerIndex) false SelectedPair))))

(fn `AddPlayerInQueue`
  (returns (PlayerIndex :type Integer))
  (locals (CurPlayerIndex :type Integer))
  (bind _playersready (`self.PlayersReady`))
  (bind _output_get (set `local.CurPlayerIndex` (`BlueprintMapLibrary.Map_Length` _playersready)))
  (`BlueprintMapLibrary.Map_Add` _playersready _output_get)
  (return (`local.CurPlayerIndex`)))

(fn `AreAllPlayersConnected`
  (returns (ReturnValue :type Boolean))
  (return (== (`BlueprintMapLibrary.Map_Length` (`self.PlayersReady`)) (`self.PlayerCount`))))

(fn `ArePlayersReady`
  (returns (AreReady :type Boolean))
  (bind _values (`BlueprintMapLibrary.Map_Values` (`self.PlayersReady`)))
  (return (not (`KismetArrayLibrary.Array_Contains` _values))))

(fn `CheckVictoryConditions`
  (returns (GameFinished :type Boolean) (PlayerLost :type Integer))
  (locals (Result :type Boolean))
  (bind _remainingplayerindices (`/Game/GameBP/Blueprints/Gameplay/Base/GS_Classic_Base.GetPlayersRemaining` (`self.GameStateRef`)))
  (bind _output (`|GetArrayItem` _remainingplayerindices))
  (if (> (`KismetArrayLibrary.Array_Length` _remainingplayerindices) 1)
    (set `local.Result` false)
    (else
      (set `local.Result` (`/Game/GameBP/Blueprints/Gameplay/Objects/O_CardMaster.HasOnlyDonkeyCard` (`self.CardMaster`) _output))))
  (return (`local.Result`) _output))

(fn `ChoosePlayerStart`
  (params (Player :type "Controller Object Reference"))
  (returns (ReturnValue :type "Actor Object Reference"))
  (locals (CurPlayerStart :type "PlayerStart Object Reference"))
  (bind _curplayertospawn (`self.CurPlayerToSpawn`))
  (if (== (`KismetArrayLibrary.Array_Length` (`self.PlayerStarts`)) 0)
    (bind _outactors (`GameplayStatics.GetAllActorsOfClass` "/Script/Engine.PlayerStart"))
    (set `self.PlayerStarts` _outactors))
  (for _array_element (`self.PlayerStarts`)
    (bind _output_get (set `local.CurPlayerStart` _array_element))
    (if (== (`PlayerStart.PlayerStartTag` _output_get) (`KismetStringLibrary.Conv_StringToName` (`KismetStringLibrary.Conv_IntToString` _curplayertospawn)))
      (`/Engine/EditorBlueprintResources/StandardMacros.IncrementInt` _curplayertospawn
        (:`  `
          (break)))))
  (return _output_get))

(fn `GetPlayerByIndex`
  (params (PlayerIndex :type Integer))
  (returns (PController :type "/Game/GameBP/Blueprints/Gameplay/Base/PC_Classic_Base Object Reference"))
  (bind _aspc_classic_base (cast `/Game/GameBP/Blueprints/Gameplay/Base/PC_Classic_Base` (`GameplayStatics.GetPlayerController` 0)))
  (return _aspc_classic_base))

(fn `IsValidCullAttempt`
  (params (PlayerIndex :type Integer) (CardPair :type "/Game/GameData/Data/Gameplay/ST_Selection_CardPair Structure"))
  (returns (ReturnValue :type Boolean))
  (bind _cardmaster (`self.CardMaster`))
  (bind _carddata_label (break `/Game/GameData/Data/Gameplay/ST_ClassicCard` (`/Game/GameBP/Blueprints/Gameplay/Objects/O_CardMaster.GetCardForPlayer` _cardmaster PlayerIndex CardPair_SecondPosition_8_94F7849946351D7164DBBDA1C493D262)))
  (bind _carddata_label_2 (break `/Game/GameData/Data/Gameplay/ST_ClassicCard` (`/Game/GameBP/Blueprints/Gameplay/Objects/O_CardMaster.GetCardForPlayer` _cardmaster PlayerIndex CardPair_FirstPosition_7_4F9BDCE74DE6C9A88ABD5F9AEC7FCC31)))
  (return (== _carddata_label_2 _carddata_label)))

(fn `LoadGameRules`
  (params (PlayerCount :type Integer))
  (switch `int` PlayerCount
    (:`1`
      ;[0.5417 0.01128 0.01128] TEMP DEV
      (bind _returnvalue (`|GetDataTableRow` "/Game/GameData/Data/Gameplay/DT_GameRules.DT_GameRules" "3")
        (:`then`
          (set `self.GameRule` _returnvalue))))
    (:`2`
      (bind _returnvalue_2 (`|GetDataTableRow` "/Game/GameData/Data/Gameplay/DT_GameRules.DT_GameRules" "0")
        (:`then`
          (set `self.GameRule` _returnvalue_2))))
    (:`3`
      (bind _returnvalue_3 (`|GetDataTableRow` "/Game/GameData/Data/Gameplay/DT_GameRules.DT_GameRules" "1")
        (:`then`
          (set `self.GameRule` _returnvalue_3))))
    (:`4`
      (bind _returnvalue_4 (`|GetDataTableRow` "/Game/GameData/Data/Gameplay/DT_GameRules.DT_GameRules" "2")
        (:`then`
          (set `self.GameRule` _returnvalue_4))))))

(fn `ResetPlayerReady`
  (params (PlayerIndex :type Integer))
  (`BlueprintMapLibrary.Map_Add` (`self.PlayersReady`) PlayerIndex))

(fn `SetPlayerReady`
  (params (PlayerIndex :type Integer))
  (bind _values (`BlueprintMapLibrary.Map_Values` (`self.PlayersReady`)))
  (if (not (`KismetArrayLibrary.Array_Contains` _values true))
    (set `self.FirstPlayerReady` PlayerIndex))
  (`BlueprintMapLibrary.Map_Add` (`self.PlayersReady`) PlayerIndex true))

(fn `UpdateCardRepositioning`
  (params (PlayerIndex :type Integer) (CardsRepositioned :type "Array of /Game/GameData/Data/Gameplay/ST_Selection_CardPair Structure"))
  (locals (CurDeck :type "/Game/GameBP/Blueprints/Gameplay/Objects/O_CardDeck Object Reference"))
  (set `local.CurDeck` (`/Game/GameBP/Blueprints/Gameplay/Objects/O_CardMaster.GetDeckForPlayer` (`self.CardMaster`) PlayerIndex))
  (for _array_element CardsRepositioned
    (bind (_firstlabel _secondlabel _firstposition _secondposition) (break `/Game/GameData/Data/Gameplay/ST_Selection_CardPair` _array_element))
    (`/Game/GameBP/Blueprints/Gameplay/Objects/O_CardDeck.RepositionCard` (`local.CurDeck`) _firstposition _secondposition))
  (return))

(fn `UpdatePlayerConnected`
  (params (PlayerIndex :type Integer) (PlayerName :type String))
  (`KismetArrayLibrary.Array_Set` (`/Game/GameBP/Blueprints/Gameplay/Base/GS_Classic_Base.PlayerNames` (`self.GameStateRef`)) PlayerIndex PlayerName true))

(fn `UserConstructionScript`)