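; Server game mode for a multiplayer Donkey card game, where players cull pairs and draw from each other until the loser holds the donkey card.
; It queues players, loads player-count rules from a DataTable and deals through an O_CardMaster that holds every hand.
; It validates culls and picks, relays them to each PC_Classic, and drives GS_Classic phases, turns and finishes.
; It reopens the server level once everyone leaves.
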(event `self.ReceiveBeginPlay`
  ;[1 1 1] BeginPlay - Get references
  (bind _asgs_classic (cast `/Game/GameBP/Blueprints/Gameplay/GS_Classic` (`GameplayStatics.GetGameState`)))
  (set `self.GameStateRef` _asgs_classic)
  (bind _asgi_core (cast `/Game/GameBP/Blueprints/GI_Core` (`GameplayStatics.GetGameInstance`)))
  (set `self.GameInstanceRef` _asgi_core)
  (bind _returnvalue (`|GenericCreateObject` "/Game/GameBP/Blueprints/Gameplay/Objects/O_CardMaster.O_CardMaster_C" self))
  (set `self.CardMaster` _returnvalue))

(event `Event Players Connected`
  ;[1 0.5744 0.09237] TODO: When matchmaking works, this should deprecate the solution below since  the server will know beforehand how many players are connected (matchmaking rule)
)

(event `self.K2_PostLogin`
  (params (NewPlayer :type "PlayerController Object Reference"))
  ;[1 0.5744 0.09237] TODO: When matchmaking works, this should deprecate the solution below since  the server will know beforehand how many players are connected (matchmaking rule)
  (bind _playerindex (`self.AddPlayerInQueue`))
  (`/Game/GameBP/Blueprints/Gameplay/PC_Classic.Event Matched` (`self.GetPlayerByIndex` _playerindex) _playerindex))

(event `self.K2_OnLogout`
  (params (ExitingController :type "Controller Object Reference"))
  ;[1 0.5744 0.09237] TODO: When matchmaking works, this should deprecate the solution below since  the server will know beforehand how many players are connected (matchmaking rule)
  ;;[0.5417 0.01128 0.01128] Player is disconnected
  (bind _asplayer_controller (cast `PlayerController` ExitingController))
  (`self.RemovePlayerFromQueue` (`AdvancedSessionsLibrary.GetNetPlayerIndex` _asplayer_controller))
  (bind _result (`/Engine/EditorBlueprintResources/StandardMacros.DecrementInt` (`self.PlayerCount`))
    (:`  `
      (if (== _result 0)
        (`GameplayStatics.OpenLevel` (`self.ServerLevelName`))))))

(event `Event Matched Player`
  (params (DesiredMatchSize :type Integer))
  (bind _cardmaster (`self.CardMaster`))
  (bind (_gamerule_id _gamerule_playercount _gamerule_cardrepetition) (break `/Game/GameData/Data/Gameplay/ST_GameRule` (`self.GameRule`)))
  ;[1 0.5744 0.09237] TODO: When matchmaking works, this should deprecate the solution below since  the server will know beforehand how many players are connected (matchmaking rule)
  (bind _isavailable (`self.IsMatchSizeAvailable` DesiredMatchSize))
  (if _isavailable
    (if (`self.AreAllPlayersConnected`)
      ;;[0.5417 0.01128 0.01128] DEV - delay for local play (to wait for BeginPlay)
      (`KismetSystemLibrary.Delay` 1.0)
      (`self.LoadGameRules` (`self.PlayerCount`))
      (`/Game/GameBP/Blueprints/Gameplay/Objects/O_CardMaster.Setup Cards For Players` _cardmaster _gamerule_playercount _gamerule_cardrepetition)
      (`KismetSystemLibrary.Delay` 1.0)
      (for _index (range (`self.PlayerCount`))
        (`/Game/GameBP/Blueprints/Gameplay/PC_Classic.Event Connected` (`self.GetPlayerByIndex` _index) (`/Game/GameBP/Blueprints/Gameplay/Objects/O_CardMaster.GetDecksForPlayer` _cardmaster _index)))
      (else
        (`KismetSystemLibrary.PrintString` "Not enough players connected")))
    (else
      (`KismetSystemLibrary.PrintString` "No Match available for that size"))))

(event `Event Player Ready`
  (params (PlayerIndex :type Integer))
  ;[1 0.5744 0.09237] TODO: When matchmaking works, this should deprecate the solution below since  the server will know beforehand how many players are connected (matchmaking rule)
  (`self.SetPlayerReady` PlayerIndex)
  (if (`self.ArePlayersReady`)
    (`self.ResetPlayersReady`)
    (`/Game/GameBP/Blueprints/Gameplay/GS_Classic.Event Begin Culling` (`self.GameStateRef`))))

(event `Event Player Repositioned Cards`
  (params (PlayerIndex :type Integer) (SubjectCardIndex :type Integer) (TargetCardIndex :type Integer))
  ;[1 1 1] Player made card reposition request -- update CardMaster
  (`/Game/GameBP/Blueprints/Gameplay/Objects/O_CardDeck.RepositionCard` (`/Game/GameBP/Blueprints/Gameplay/Objects/O_CardMaster.GetDeckForPlayer` (`self.CardMaster`) PlayerIndex) SubjectCardIndex TargetCardIndex))

(event `Event Player Picked Card`
  (params (CardIndex :type Integer))
  (bind (_gamerule_id _gamerule_playercount _gamerule_cardrepetition _gamerule_timeperturn) (break `/Game/GameData/Data/Gameplay/ST_GameRule` (`self.GameRule`)))
  (bind _gamestateref (`self.GameStateRef`))
  (bind _gamestateref_2 (`self.GameStateRef`))
  (bind _gamestateref_3 (`self.GameStateRef`))
  (bind _cardmaster (`self.CardMaster`))
  (bind _activeplayerindex (`/Game/GameBP/Blueprints/Gameplay/GS_Classic.ActivePlayerIndex` _gamestateref))
  (bind _nextplayerindex (`/Game/GameBP/Blueprints/Gameplay/GS_Classic.NextPlayerIndex` _gamestateref))
  (bind _nextplayerindex_2 (`/Game/GameBP/Blueprints/Gameplay/GS_Classic.NextPlayerIndex` _gamestateref_2))
  (bind _nextplayerindex_3 (`/Game/GameBP/Blueprints/Gameplay/GS_Classic.NextPlayerIndex` _gamestateref_3))
  (bind _activeplayerindex_2 (`/Game/GameBP/Blueprints/Gameplay/GS_Classic.ActivePlayerIndex` _gamestateref_3))
  (bind _carddata (`/Game/GameBP/Blueprints/Gameplay/Objects/O_CardMaster.GetCardForPlayer` _cardmaster _nextplayerindex_3 CardIndex))
  ;[1 1 1] Player picked a card from the next player -- End turn
  (`/Game/GameBP/Blueprints/Gameplay/PC_Classic.Event Card Added` (`self.GetPlayerByIndex` _activeplayerindex_2) _carddata)
  (`/Game/GameBP/Blueprints/Gameplay/Objects/O_CardMaster.AddCardForPlayer` _cardmaster _activeplayerindex_2 _carddata)
  (`/Game/GameBP/Blueprints/Gameplay/PC_Classic.Event Card Removed` (`self.GetPlayerByIndex` _nextplayerindex_3) CardIndex)
  (`/Game/GameBP/Blueprints/Gameplay/Objects/O_CardMaster.RemoveCardForPlayer` (`self.CardMaster`) _nextplayerindex_3 CardIndex)
  (for _index (range (`self.PlayerCount`))
    (`|ExecutionSequence`
      (:`then_0`
        (if (!= _index _activeplayerindex)
          (bind _aspc_classic (`self.GetPlayerByIndex` _index))
          (`/Game/GameBP/Blueprints/Gameplay/PC_Classic.Event Other PC Added Card` _aspc_classic (make `/Game/GameData/Data/Gameplay/ST_AddedCard` _activeplayerindex))))
      (:`then_1`
        (if (!= _index _nextplayerindex)
          (`/Game/GameBP/Blueprints/Gameplay/PC_Classic.Event Other PC Removed Card` _aspc_classic (make `/Game/GameData/Data/Gameplay/ST_RemovedCard` _nextplayerindex CardIndex))))))
  ;[1 1 1] Check if the BeingPicked player has remaining cards in hand -- Next Turn
  (if (`/Game/GameBP/Blueprints/Gameplay/Objects/O_CardMaster.Has Remaining Cards For Player` (`self.CardMaster`) _nextplayerindex_2)
    (`/Game/GameBP/Blueprints/Gameplay/GS_Classic.Event Next Turn` _gamestateref_2 (`KismetMathLibrary.Conv_IntToDouble` _gamerule_timeperturn))
    (else
      (`/Game/GameBP/Blueprints/Gameplay/GS_Classic.Event Player Finished` _gamestateref_2 _nextplayerindex_2 false true (`KismetMathLibrary.Conv_IntToDouble` _gamerule_timeperturn)))))

(event `Event Player Culled Cards`
  (params (PlayerIndex :type Integer) (SelectedPair :type "/Game/GameData/Data/Gameplay/ST_Selection_CardPair Structure"))
  (bind (_firstlabel _secondlabel) (break `/Game/GameData/Data/Gameplay/ST_Selection_CardPair` SelectedPair))
  (bind (_gamefinished _playerlost) (`self.CheckVictoryConditions`))
  (bind _aspc_classic (`self.GetPlayerByIndex` PlayerIndex))
  ;[1 1 1] Player has selected two cards to cull
  (if (== _firstlabel _secondlabel)
    (`/Game/GameBP/Blueprints/Gameplay/Objects/O_CardMaster.RemoveCardPair` (`self.CardMaster`) PlayerIndex SelectedPair)
    (`/Game/GameBP/Blueprints/Gameplay/PC_Classic.Event Cards Culled` _aspc_classic true SelectedPair)
    (for _index (range (`self.PlayerCount`))
      (if (!= _index PlayerIndex)
        (`/Game/GameBP/Blueprints/Gameplay/PC_Classic.Event Other Player Culled` (`self.GetPlayerByIndex` _index) PlayerIndex SelectedPair)))
    (switch `/Game/GameData/Data/Enums/E_GamePhases` (`/Game/GameBP/Blueprints/Gameplay/GS_Classic.GamePhase` (`self.GameStateRef`))
      (:`NewEnumerator0`
        ;[1 1 1] Check for remaining pairs -- if all players finished, tell GS to end the Culling phase
        (if (not (`/Game/GameBP/Blueprints/Gameplay/Objects/O_CardMaster.Has Remaining Pairs For Player` (`self.CardMaster`) PlayerIndex))
          (`self.SetPlayerReady` PlayerIndex)
          (if (`self.ArePlayersReady`)
            (`/Game/GameBP/Blueprints/Gameplay/GS_Classic.Event Begin RoundTable` (`self.GameStateRef`) 0 (`self.PlayerCount`)))))
      (:`NewEnumerator1`
        ;[1 1 1] Check if player who culled has remaining cards in hand
        (if (not (`/Game/GameBP/Blueprints/Gameplay/Objects/O_CardMaster.Has Remaining Cards For Player` (`self.CardMaster`) PlayerIndex)) :!label _label
          (`/Game/GameBP/Blueprints/Gameplay/GS_Classic.Event Player Finished` (`self.GameStateRef`) PlayerIndex false false 0.0))
        ;[1 1 1] Check for Finished Game
        (if _gamefinished
          (`/Game/GameBP/Blueprints/Gameplay/GS_Classic.Event Player Finished` (`self.GameStateRef`) _playerlost true false 0.0)))
      (:`NewEnumerator2`
        (goto _label)))
    (else
      (`/Game/GameBP/Blueprints/Gameplay/PC_Classic.Event Cards Culled` _aspc_classic false SelectedPair))))

(fn `AddPlayerInQueue`
  (returns (PlayerIndex :type Integer))
  (locals (CurPlayerIndex :type Integer :default 0))
  (bind _playersready (`self.PlayersReady`))
  (bind _output_get (set `local.CurPlayerIndex` (`BlueprintMapLibrary.Map_Length` _playersready)))
  (`BlueprintMapLibrary.Map_Add` _playersready _output_get)
  (return (`local.CurPlayerIndex`)))

(fn `AreAllPlayersConnected`
  (returns (ReturnValue :type Boolean))
  (bind _returnvalue (`self.GetNumPlayers`))
  (return (== _returnvalue (`self.PlayerCount`))))

(fn `ArePlayersReady`
  (returns (AreReady :type Boolean))
  (bind _values (`BlueprintMapLibrary.Map_Values` (`self.PlayersReady`)))
  (return (not (`KismetArrayLibrary.Array_Contains` _values))))

(fn `CheckVictoryConditions`
  (returns (GameFinished :type Boolean) (PlayerLost :type Integer))
  (locals (Result :type Boolean))
  (bind _remainingplayerindices (`/Game/GameBP/Blueprints/Gameplay/GS_Classic.GetPlayersRemaining` (`self.GameStateRef`)))
  (bind _output (`|GetArrayItem` _remainingplayerindices))
  (if (> (`KismetArrayLibrary.Array_Length` _remainingplayerindices) 1)
    (set `local.Result` false)
    (else
      (set `local.Result` (`/Game/GameBP/Blueprints/Gameplay/Objects/O_CardMaster.HasOnlyDonkeyCard` (`self.CardMaster`) _output))))
  (return (`local.Result`) _output))

(fn `ChoosePlayerStart`
  (params (Player :type "Controller Object Reference"))
  (returns (ReturnValue :type "Actor Object Reference"))
  (locals (CurPlayerStart :type "PlayerStart Object Reference"))
  (bind _curplayertospawn (`self.CurPlayerToSpawn`))
  (if (== (`KismetArrayLibrary.Array_Length` (`self.PlayerStarts`)) 0)
    (bind _outactors (`GameplayStatics.GetAllActorsOfClass` "/Script/Engine.PlayerStart"))
    (set `self.PlayerStarts` _outactors))
  (for _array_element (`self.PlayerStarts`)
    (bind _output_get (set `local.CurPlayerStart` _array_element))
    (if (== (`PlayerStart.PlayerStartTag` _output_get) (`KismetStringLibrary.Conv_StringToName` (`KismetStringLibrary.Conv_IntToString` _curplayertospawn)))
      (`/Engine/EditorBlueprintResources/StandardMacros.IncrementInt` _curplayertospawn
        (:`  `
          (break)))))
  (return _output_get))

(fn `GetPlayerByIndex`
  (params (PlayerIndex :type Integer))
  (returns (`AsPC Classic` :type "/Game/GameBP/Blueprints/Gameplay/PC_Classic Object Reference"))
  (bind _aspc_classic (cast `/Game/GameBP/Blueprints/Gameplay/PC_Classic` (`GameplayStatics.GetPlayerController` PlayerIndex)))
  (return _aspc_classic))

(fn `IsMatchSizeAvailable`
  (params (DesiredSize :type Integer))
  (returns (IsAvailable :type Boolean))
  (locals (Result :type Boolean :default false))
  (if (== (`self.PlayerCount`) -1)
    (set `self.PlayerCount` DesiredSize)
    (set `local.Result` true)
    (else
      (set `local.Result` (== DesiredSize (`self.PlayerCount`)))))
  (return (`local.Result`)))

(fn `LoadGameRules`
  (params (PlayerCount :type Integer))
  (switch `int` PlayerCount
    (:`1`
      ;[0.5417 0.01128 0.01128] TEMP DEV
      (bind _returnvalue (`|GetDataTableRow` "/Game/GameData/Data/Gameplay/DT_GameRules.DT_GameRules" "3")
        (:`then`
          (set `self.GameRule` _returnvalue))))
    (:`2`
      (bind _returnvalue_2 (`|GetDataTableRow` "/Game/GameData/Data/Gameplay/DT_GameRules.DT_GameRules" "0")
        (:`then`
          (set `self.GameRule` _returnvalue_2))))
    (:`3`
      (bind _returnvalue_3 (`|GetDataTableRow` "/Game/GameData/Data/Gameplay/DT_GameRules.DT_GameRules" "1")
        (:`then`
          (set `self.GameRule` _returnvalue_3))))
    (:`4`
      (bind _returnvalue_4 (`|GetDataTableRow` "/Game/GameData/Data/Gameplay/DT_GameRules.DT_GameRules" "2")
        (:`then`
          (set `self.GameRule` _returnvalue_4))))))

(fn `RemovePlayerFromQueue`
  (params (Index :type Integer))
  (locals (CurPlayerIndex :type Integer :default 0))
  (`BlueprintMapLibrary.Map_Remove` (`self.PlayersReady`) Index)
  (return))

(fn `ResetPlayersReady`
  (for _index (range (`self.PlayerCount`))
    (`BlueprintMapLibrary.Map_Add` (`self.PlayersReady`) _index))
  (return))

(fn `SetPlayerReady`
  (params (PlayerIndex :type Integer))
  (`BlueprintMapLibrary.Map_Add` (`self.PlayersReady`) PlayerIndex true))

(fn `UserConstructionScript`)