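; BP_GameBoard_01 is a game board actor that animates its environment, currently a mill with rotating blades.
; After the parent BeginPlay and a short delay, it fires an environment animation event that starts the mill animation.
; A timeline drives the blades' relative roll each update while holding pitch and yaw fixed.
; The construction script only calls its parent.
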(event `self.ReceiveBeginPlay`
  (`parent.ReceiveBeginPlay`)
  (`KismetSystemLibrary.Delay` 2.0)
  (`self.Event Animate Environment`))

(event `Event Animate Environment`
  (`self.Event Animate Mill`))

(event `Event Animate Mill`
  (bind (_direction _rotationofmillbladex) (`Timeline|Timeline_RotateMillBlades` :!via `PlayFromStart`)
    (:`Update`
      (`SceneComponent.K2_SetRelativeRotation` (`self.MillBlades`) (`KismetMathLibrary.MakeRotator` _rotationofmillbladex 0.0 -105.0) false false))))

(fn `UserConstructionScript`
  (`parent.UserConstructionScript`))