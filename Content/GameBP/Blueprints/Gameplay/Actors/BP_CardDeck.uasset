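; Actor that displays a card deck as a row of BP_Card child actors and handles adding, removing, pair culling and repositioning.
; It mirrors changes into the CardDeck data object, keeps an index-ordered component array and dispatches count changes.
; Cards form an attachment chain, the first on CardHolder and each other on its predecessor, so edits re-index and re-link only affected neighbors.
; Enemy decks drop their deck collision.
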(event `Event Create With Data`
  (params (DeckIndex :type Integer) (CardDeck :type "/Game/GameBP/Blueprints/Gameplay/Objects/O_CardDeck Object Reference"))
  ;[1 1 1] Spawn cards
  (bind _aspc_classic (cast `/Game/GameBP/Blueprints/Gameplay/PC_Classic` (`GameplayStatics.GetPlayerController` 0)))
  (set `self.PlayerControllerRef` _aspc_classic)
  (set `self.DeckIndex` DeckIndex)
  (bind _output_get (set `self.CardDeck` CardDeck))
  (cast `/Game/GameBP/Blueprints/Gameplay/Objects/O_EnemyDeck` _output_get
    (:`then`
      (`self.ConfigForEnemyDeck`))
    (:`CastFailed`
      _))
  (bind _cards (`/Game/GameBP/Blueprints/Gameplay/Objects/O_CardDeck.GetCards` _output_get))
  (set `self.Size` (`KismetArrayLibrary.Array_Length` _cards))
  (for (_array_element _array_index) _cards
    (`self.CreateCardComponent` _array_element _array_index)
    (`self.DispatchCardAddedToDeck` (`self.DeckIndex`))))

(event `Event Cull Cards`
  (params (CardPair :type "/Game/GameData/Data/Gameplay/ST_Selection_CardPair Structure"))
  (bind (_firstlabel _secondlabel _firstposition _secondposition) (break `/Game/GameData/Data/Gameplay/ST_Selection_CardPair` CardPair))
  ;[1 1 1] The Culling phase -- cull cards at selected indices
  (`self.SetComponentToAttach` _firstposition)
  (`self.SetComponentToAttach` _secondposition)
  (`self.Remove Card Pair` CardPair)
  (`self.AttachComponentToRoot`)
  (`self.UpdateCardActorPositions` CardPair)
  (`self.DispatchCardRemovedFromDeck` (`self.DeckIndex`) 2))

(event `Event Bad Cull Attempt`
  (params (CardPair :type "/Game/GameData/Data/Gameplay/ST_Selection_CardPair Structure"))
  ;[1 1 1] The Culling phase -- cull cards at selected indices
  (`/Game/GameBP/Blueprints/Gameplay/Actors/BP_Card.Deselect` (`self.Get Card As Actor` CardPair_FirstPosition_7_4F9BDCE74DE6C9A88ABD5F9AEC7FCC31))
  (`/Game/GameBP/Blueprints/Gameplay/Actors/BP_Card.Deselect` (`self.Get Card As Actor` CardPair_SecondPosition_8_94F7849946351D7164DBBDA1C493D262)))

(event `Event Removed Card`
  (params (CardIndex :type Integer))
  ;[1 1 1] Event Card Removed/Added
  (`self.SetComponentToAttach` CardIndex)
  (`self.Remove Card` CardIndex)
  (`self.Update Cards Indices`)
  (`self.AttachComponentToRoot`)
  (`self.UpdateCardActorPosition` CardIndex)
  (`self.DispatchCardRemovedFromDeck` (`self.DeckIndex`) 1))

(event `Event Reposition Cards`
  (params (SubjectCardPos :type Integer) (TargetCardPos :type Integer))
  ;[1 0.5744 0.09237] TODO: This should happen once card is confirmed for repositioning (i.e: card released on specifried pos)
  (`self.MoveCardComponentPos` SubjectCardPos TargetCardPos)
  (`self.Update Cards Indices`)
  (`self.UpdateCardActorPosition` (+ TargetCardPos 1)) ; attach next card to +1 pos
  (`self.UpdateCardActorPosition` TargetCardPos) ; attach subj card at new pos
  (if (== SubjectCardPos 0)
    (`/Game/GameBP/Blueprints/Gameplay/Actors/BP_Card.MoveInDirection` (`self.Get Card As Actor` SubjectCardPos) "Left" (`self.Card Attach Distance`)) ; shift first card back to position
    (else
      (`self.UpdateCardActorPosition` SubjectCardPos) ; attach card left at subj pos
    ))
  (`/Game/GameBP/Blueprints/Gameplay/Objects/O_CardDeck.RepositionCard` (`self.CardDeck`) SubjectCardPos TargetCardPos))

(event `Event Added Card`
  (params (CardData :type "/Game/GameData/Data/Gameplay/ST_ClassicCard Structure"))
  ;[1 1 1] Event Card Removed/Added
  (`self.AddNewCard` CardData)
  (`self.DispatchCardAddedToDeck` (`self.DeckIndex`)))

(fn `AddNewCard`
  (params (CardData :type "/Game/GameData/Data/Gameplay/ST_ClassicCard Structure"))
  (bind _size (`self.Size`))
  (`/Game/GameBP/Blueprints/Gameplay/Objects/O_CardDeck.AddCard` (`self.CardDeck`) CardData)
  (`self.CreateCardComponent` CardData _size)
  (`/Engine/EditorBlueprintResources/StandardMacros.IncrementInt` _size))

(fn `AttachCardToRoot`
  (params (CardPos :type Integer))
  (bind _component (`self.GetCardAsComponent` CardPos))
  (`/Engine/EditorBlueprintResources/StandardMacros.IsValid` _component
    (:`Is Valid`
      (`SceneComponent.K2_AttachToComponent` _component (`self.CardHolder`) "None" "KeepRelative" "KeepRelative" "KeepRelative" false))))

(fn `AttachComponentToRoot`
  (`/Engine/EditorBlueprintResources/StandardMacros.IsValid` (`self.TempComponentToAttach`)
    (:`Is Valid`
      (`SceneComponent.K2_AttachToComponent` (`self.TempComponentToAttach`) (`self.CardHolder`) "None" "KeepRelative" "KeepRelative" "KeepRelative" false)
      (set `self.TempComponentToAttach` null))))

(fn `ConfigForEnemyDeck`
  (`ActorComponent.K2_DestroyComponent` (`self.DeckCollision`)))

(fn `CreateCardComponent`
  (params (CardData :type "/Game/GameData/Data/Gameplay/ST_ClassicCard Structure") (IndexInHand :type Integer))
  (bind _returnvalue (`|AddComponentByClass` "/Script/Engine.ChildActorComponent" true))
  (`ChildActorComponent.SetChildActorClass` _returnvalue "/Game/GameBP/Blueprints/Gameplay/Actors/BP_Card.BP_Card_C")
  (`SceneComponent.K2_AttachToComponent` _returnvalue (`self.CardHolder`) "None" "KeepRelative" "KeepRelative" "KeepRelative" true)
  (`self.PushCardComponent` _returnvalue)
  (`/Game/GameBP/Blueprints/Gameplay/Actors/BP_Card.Create` (`self.Get Card As Actor` IndexInHand) CardData IndexInHand (`self.Card Attach Distance`) (`self.Card Attach Height`))
  (if (> IndexInHand 0)
    (`self.UpdateCardActorPosition` IndexInHand)))

(fn `DestroyCardAtPos`
  (params (ChildIndex :type Integer))
  (`ActorComponent.K2_DestroyComponent` (`self.GetCardAsComponent` ChildIndex))
  (`KismetArrayLibrary.Array_Remove` (`self.ComponentsByIndex`) ChildIndex))

(fn `Get Card As Actor`
  (params (Position :type Integer))
  (returns (`AsBP Card` :type "/Game/GameBP/Blueprints/Gameplay/Actors/BP_Card Object Reference"))
  (bind _asbp_card (`self.ComponentToCard` (`self.GetCardAsComponent` Position)))
  (return _asbp_card))

(fn `GetCardAsComponent`
  (params (ChildIndex :type Integer))
  (returns (Component :type "ChildActorComponent Object Reference"))
  (bind _componentsbyindex (`self.ComponentsByIndex`))
  (if (`KismetArrayLibrary.Array_IsValidIndex` _componentsbyindex ChildIndex)
    (return (`|GetArrayItem` _componentsbyindex ChildIndex))
    (else
      (return null))))

(fn `MoveCardComponentPos`
  (params (SubjectCardPos :type Integer) (TargetPos :type Integer))
  (locals (CurCardComponent :type "ChildActorComponent Object Reference"))
  (bind _componentsbyindex (`self.ComponentsByIndex`))
  (`KismetArrayLibrary.Array_Insert` _componentsbyindex (`|GetArrayItem` _componentsbyindex SubjectCardPos) TargetPos)
  (`KismetArrayLibrary.Array_Remove` _componentsbyindex SubjectCardPos))

(fn `PushCardComponent`
  (params (CardComponent :type "ChildActorComponent Object Reference (by ref)"))
  (`KismetArrayLibrary.Array_Add` (`self.ComponentsByIndex`) CardComponent))

(fn `Remove Card`
  (params (Position :type Integer))
  (`/Game/GameBP/Blueprints/Gameplay/Objects/O_CardDeck.RemoveCardAtPos` (`self.CardDeck`) Position)
  (`self.DestroyCardAtPos` Position)
  (`/Engine/EditorBlueprintResources/StandardMacros.DecrementInt` (`self.Size`)))

(fn `Remove Card Pair`
  (params (CardPair :type "/Game/GameData/Data/Gameplay/ST_Selection_CardPair Structure"))
  (locals (CardToDestroy1 :type "SceneComponent Object Reference") (CardToDestroy2 :type "SceneComponent Object Reference"))
  (bind (_firstlabel _secondlabel _firstposition _secondposition) (break `/Game/GameData/Data/Gameplay/ST_Selection_CardPair` CardPair))
  (`/Engine/EditorBlueprintResources/StandardMacros.CompareInt` _firstposition _secondposition ; Make sure the biggest pos is removed first
    (:`>`
      (`self.Remove Card` _firstposition)
      (`self.Remove Card` _secondposition))
    (:`<`
      (`self.Remove Card` _secondposition)
      (`self.Remove Card` _firstposition)))
  (`self.Update Cards Indices`))

(fn `SetComponentToAttach`
  (params (CardIndexRemoved :type Integer))
  (if (== CardIndexRemoved 0)
    (set `self.TempComponentToAttach` (`self.GetCardAsComponent` 1))))

(fn `Shift from Card`
  (params (Card :type "/Game/GameBP/Blueprints/Gameplay/Actors/BP_Card Object Reference") (Direction :type "ETouchSwipeDirection Enum" :default "None"))
  (`/Game/GameBP/Blueprints/Gameplay/Actors/BP_Card.MoveInDirection` Card Direction (`self.Card Attach Distance`)) ; TODO: Should interpolate
)

(fn `Update Cards Indices`
  (for (_array_element _array_index) (`self.ComponentsByIndex`)
    (bind _asbp_card (`self.ComponentToCard` _array_element))
    (set `/Game/GameBP/Blueprints/Gameplay/Actors/BP_Card.IndexInHand` _array_index _asbp_card)
    (`/Game/GameBP/Blueprints/Gameplay/Actors/BP_Card.DEBUG_RenderIndex` _asbp_card)))

(fn `UpdateCardActorPosition`
  (params (RemovedCardIndex :type Integer))
  (locals (FirstIndexToMove :type Integer :default -1) (SecondIndexToMove :type Integer :default -1))
  (if (== RemovedCardIndex 0)
    (set `self.TempComponentToAttach` (`self.GetCardAsComponent` 0))
    (`self.AttachComponentToRoot`)
    (else
      (`self.ValidateAndAttachCards` RemovedCardIndex (- RemovedCardIndex 1)
        (:`Continue`
          _))))
  (return))

(fn `UpdateCardActorPositions`
  (params (PairRemoved :type "/Game/GameData/Data/Gameplay/ST_Selection_CardPair Structure"))
  (locals (FirstIndexToMove :type Integer :default -1) (SecondIndexToMove :type Integer :default -1))
  (bind _returnvalue (`KismetMathLibrary.Min` PairRemoved_FirstPosition_7_4F9BDCE74DE6C9A88ABD5F9AEC7FCC31 PairRemoved_SecondPosition_8_94F7849946351D7164DBBDA1C493D262))
  (bind _secondindextomove (`local.SecondIndexToMove`))
  (bind _firstindextomove (`local.FirstIndexToMove`))
  (if (== (`KismetMathLibrary.Abs_Int` (- PairRemoved_FirstPosition_7_4F9BDCE74DE6C9A88ABD5F9AEC7FCC31 PairRemoved_SecondPosition_8_94F7849946351D7164DBBDA1C493D262)) 1)
    (`self.ValidateAndAttachCards` _returnvalue (- _returnvalue 1))
    (else
      (`|ExecutionSequence`
        (:`then_0`
          (set `local.FirstIndexToMove` (- (`KismetMathLibrary.Max` PairRemoved_FirstPosition_7_4F9BDCE74DE6C9A88ABD5F9AEC7FCC31 PairRemoved_SecondPosition_8_94F7849946351D7164DBBDA1C493D262) 1)))
        (:`then_1`
          (set `local.SecondIndexToMove` (`KismetMathLibrary.Min` PairRemoved_FirstPosition_7_4F9BDCE74DE6C9A88ABD5F9AEC7FCC31 PairRemoved_SecondPosition_8_94F7849946351D7164DBBDA1C493D262)))
        (:`then_2`
          (`self.ValidateAndAttachCards` _firstindextomove (- _firstindextomove 1)))
        (:`then_3`
          (`self.ValidateAndAttachCards` _secondindextomove (- _secondindextomove 1)))))))

(fn `UserConstructionScript`
  ;[0.5417 0.01128 0.01128] DEBUGGING PURPOSES
)