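; BP_GameBoard is the table actor for a pair-culling card game with a donkey card, seating up to four players around child-actor BP_CardDecks.
; CreateWithData puts the owning player's deck at position 0, maps every player to a deck and seat, and trims unused decks, tightening card spacing for three players.
; Card add, remove and pair-cull events route to that player's deck.
; BeginPlay applies the board theme through a dynamic material.
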(event `self.ReceiveBeginPlay`
  ;[1 1 1] Begin play - references, config etc
  (`self.RenderTheme`))

(event `Event Create With Data`
  (params (Decks :type "Array of /Game/GameBP/Blueprints/Gameplay/Objects/O_CardDeck Object Reference") (OwningPlayerIndex :type Integer))
  (bind _nextfreedeckindex (`self.NextFreeDeckIndex`))
  ;[1 1 1] Create - Configure GameBoard
  (for (_array_element _array_index) Decks
    (cast `/Game/GameBP/Blueprints/Gameplay/Objects/O_PlayerDeck` _array_element
      (:`then`
        (`self.SetCardActorForPlayer` OwningPlayerIndex 0 Decks))
      (:`CastFailed`
        (bind _createddeck (`self.SetCardActorForPlayer` _array_index _nextfreedeckindex Decks))
        (`/Game/GameBP/Blueprints/Gameplay/Actors/BP_CardDeck.SetPlayerName` _createddeck (`/Game/GameBP/Blueprints/Gameplay/Objects/O_CardDeck.OwningPlayerName` _array_element))
        (`/Engine/EditorBlueprintResources/StandardMacros.IncrementInt` _nextfreedeckindex))))
  (switch `int` (`KismetArrayLibrary.Array_Length` Decks)
    (:`2`
      (`ActorComponent.K2_DestroyComponent` (`self.Deck_3`))
      (`ActorComponent.K2_DestroyComponent` (`self.Deck_2`)))
    (:`3`
      (`ActorComponent.K2_DestroyComponent` (`self.Deck_3`))
      (for _index (range 3)
        (`/Game/GameBP/Blueprints/Gameplay/Actors/BP_CardDeck.CloserCardsConfiguration` (`self.GetDeckActor` _index))))))

(event `Event Card Removed By Player`
  (params (RemovedCardDeal :type "/Game/GameData/Data/Gameplay/ST_RemovedCard Structure"))
  (bind _asbp_card_deck (`self.ComponentToDeck` (`BlueprintMapLibrary.Map_Find` (`self.DeckActorsForPlayers`) RemovedCardDeal_ByPlayerIndex_6_45AE6FF44E7A35E95F140AA3A9B0F041)))
  (`/Game/GameBP/Blueprints/Gameplay/Actors/BP_CardDeck.Event Removed Card` _asbp_card_deck RemovedCardDeal_RemovedCardIndex_7_158AF5F44CC6DAB8B69CF1B86FD078E0))

(event `Event Pair Removed By Player`
  (params (PlayerIndex :type Integer) (CardPair :type "/Game/GameData/Data/Gameplay/ST_Selection_CardPair Structure"))
  ;[1 1 1] Another player has culled cards -> update respective Deck actor
  (bind _asbp_card_deck (`self.ComponentToDeck` (`BlueprintMapLibrary.Map_Find` (`self.DeckActorsForPlayers`) PlayerIndex)))
  (`/Game/GameBP/Blueprints/Gameplay/Actors/BP_CardDeck.Event Cull Cards` _asbp_card_deck CardPair))

(event `Event Card Added By Player`
  (params (AddedCardDeal :type "/Game/GameData/Data/Gameplay/ST_AddedCard Structure"))
  ;[1 1 1] Card added on another player
  (bind _asbp_card_deck (`self.ComponentToDeck` (`BlueprintMapLibrary.Map_Find` (`self.DeckActorsForPlayers`) AddedCardDeal_ByPlayerIndex_6_45AE6FF44E7A35E95F140AA3A9B0F041)))
  (`/Game/GameBP/Blueprints/Gameplay/Actors/BP_CardDeck.Event Added Card` _asbp_card_deck AddedCardDeal_AddedCardData_5_329F116541146B5FCF1A37AB844F7FA9))

(fn `Get Seat Transform For Player`
  (params (PlayerIndex :type Integer))
  (returns (PlayerSeatTransform :type "Transform Structure"))
  (return (`SceneComponent.K2_GetComponentToWorld` (`BlueprintMapLibrary.Map_Find` (`self.SeatsForPlayers`) PlayerIndex))))

(fn `GetDeckActor`
  (params (Position :type Integer))
  (returns (Deck :type "/Game/GameBP/Blueprints/Gameplay/Actors/BP_CardDeck Object Reference"))
  (locals (CurDeck :type "/Game/GameBP/Blueprints/Gameplay/Actors/BP_CardDeck Object Reference"))
  (switch `int` Position
    (:`0`
      (bind _asbp_card_deck (`self.ComponentToDeck` (`self.Deck_0`)))
      (set `local.CurDeck` _asbp_card_deck))
    (:`1`
      (bind _asbp_card_deck_2 (`self.ComponentToDeck` (`self.Deck_1`)))
      (set `local.CurDeck` _asbp_card_deck_2))
    (:`2`
      (bind _asbp_card_deck_3 (`self.ComponentToDeck` (`self.Deck_2`)))
      (set `local.CurDeck` _asbp_card_deck_3))
    (:`3`
      (bind _asbp_card_deck_4 (`self.ComponentToDeck` (`self.Deck_3`)))
      (set `local.CurDeck` _asbp_card_deck_4)))
  (return (`local.CurDeck`)))

(fn `GetDeckActorForPlayer`
  (params (PlayerIndex :type "Integer (by ref)"))
  (returns (CardDeck :type "/Game/GameBP/Blueprints/Gameplay/Actors/BP_CardDeck Object Reference"))
  (bind _asbp_card_deck (`self.ComponentToDeck` (`BlueprintMapLibrary.Map_Find` (`self.DeckActorsForPlayers`) PlayerIndex)))
  (return _asbp_card_deck))

(fn `GetDeckComponent`
  (params (DeckIndex :type Integer))
  (returns (DeckComponent :type "ChildActorComponent Object Reference"))
  (locals (CurDeck :type "ChildActorComponent Object Reference"))
  (switch `int` DeckIndex
    (:`0`
      (set `local.CurDeck` (`self.Deck_0`)))
    (:`1`
      (set `local.CurDeck` (`self.Deck_1`)))
    (:`2`
      (set `local.CurDeck` (`self.Deck_2`)))
    (:`3`
      (set `local.CurDeck` (`self.Deck_3`))))
  (return (`local.CurDeck`)))

(fn `GetHorizontalAxisForPlayer`
  (params (PlayerIndex :type Integer))
  (returns (HorizontalAxis :type "/Game/GameData/Data/Enums/E_Axis Enum"))
  (locals (Result :type Integer :default 0) (Axis :type "/Game/GameData/Data/Enums/E_Axis Enum"))
  (switch `int` PlayerIndex
    (:`0`
      (set `local.Axis` "NewEnumerator0" :!label _label))
    (:`1`
      (set `local.Axis` "NewEnumerator1" :!label _label_2))
    (:`2`
      (goto _label_2))
    (:`3`
      (goto _label)))
  (return (`local.Axis`)))

(fn `GetNumOfDecks`
  (returns (NumberOfDecks :type Integer))
  (return (`BlueprintMapLibrary.Map_Length` (`self.DeckActorsForPlayers`))))

(fn `GetSeatComponent`
  (params (DeckIndex :type Integer))
  (returns (Seat :type "ArrowComponent Object Reference"))
  (locals (CurDeck :type "ChildActorComponent Object Reference") (CurSeat :type "ArrowComponent Object Reference"))
  (switch `int` DeckIndex
    (:`0`
      (set `local.CurSeat` (`self.Seat_0`)))
    (:`1`
      (set `local.CurSeat` (`self.Seat_1`)))
    (:`2`
      (set `local.CurSeat` (`self.Seat_2`)))
    (:`3`
      (set `local.CurSeat` (`self.Seat_3`))))
  (return (`local.CurSeat`)))

(fn `GetVerticalAxisForPlayer`
  (params (PlayerIndex :type Integer))
  (returns (VerticalAxis :type "/Game/GameData/Data/Enums/E_Axis Enum"))
  (locals (Result :type Integer :default 0) (Axis :type "/Game/GameData/Data/Enums/E_Axis Enum"))
  (switch `int` PlayerIndex
    (:`0`
      (set `local.Axis` "NewEnumerator1" :!label _label))
    (:`1`
      (set `local.Axis` "NewEnumerator0" :!label _label_2))
    (:`2`
      (goto _label_2))
    (:`3`
      (goto _label)))
  (return (`local.Axis`)))

(fn `RenderTheme`
  (bind (_boardtheme_backgroundimg _boardtheme_fronttexture) (break `/Game/GameData/Data/Gameplay/Theme/ST_BoardTheme` (`self.BoardTheme`)))
  (bind _returnvalue (`PrimitiveComponent.CreateDynamicMaterialInstance` (`self.Plane`) 0 "/Game/GameData/Materials/M_Board.M_Board" "None"))
  (bind _output_get (set `self.BoardMaterialInst` _returnvalue))
  (`MaterialInstanceDynamic.SetTextureParameterValue` _output_get "BackgroundTexture" _boardtheme_backgroundimg)
  (`MaterialInstanceDynamic.SetTextureParameterValue` _output_get "FrontTexture" _boardtheme_fronttexture))

(fn `UpdateDeckOffset`
  (params (DeckIndex :type Integer))
  (locals (ResLocation :type "Vector Structure" :default (0.0 0.0 0.0)))
  (switch `int` DeckIndex
    (:`0`
      (set `local.ResLocation` (`KismetMathLibrary.MakeVector` 0.0 1.0)))
    (:`1`
      (set `local.ResLocation` (`KismetMathLibrary.MakeVector` -1.0)))
    (:`2`
      (set `local.ResLocation` (`KismetMathLibrary.MakeVector` 1.0)))
    (:`3`
      (set `local.ResLocation` (`KismetMathLibrary.MakeVector` 0.0 -1.0)))))

(fn `UserConstructionScript`)