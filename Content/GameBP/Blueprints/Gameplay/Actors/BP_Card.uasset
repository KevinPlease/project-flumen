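; Card actor for a hand of cards, set up from card data with a label and a material swap for selection.
; Cards chain by snapping to the previous card's right join point, and enemy cards (label -1) lose their collision trigger.
; Pickup mode enables physics and detaches the join point, then restores it on release.
; Seek and move shift the dummy root instantly, with seek also resizing the trigger.
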(fn `AttachToCard`
  (params (OtherCard :type "/Game/GameBP/Blueprints/Gameplay/Actors/BP_Card Object Reference"))
  (`self.K2_AttachToComponent` (`self.GetAttachPoint` OtherCard) "None" "SnapToTarget" "SnapToTarget" "KeepWorld"))

(fn `ConfigureAttachPoints`
  (bind (_cardattachloc_x _cardattachloc_y _cardattachloc_z) (`KismetMathLibrary.BreakVector` (`self.CardAttachLoc`)))
  (`SceneComponent.K2_AttachToComponent` (`self.RightJoinPoint`) (`self.CardMesh`) "None" "KeepRelative" "KeepWorld" "KeepRelative" true)
  (`SceneComponent.K2_SetRelativeLocation` (`self.RightJoinPoint`) (`KismetMathLibrary.MakeVector` _cardattachloc_x 0.0 (* -1 _cardattachloc_z)) false false))

(fn `Create`
  (params (CardData :type "/Game/GameData/Data/Gameplay/ST_ClassicCard Structure") (IndexInHand :type Integer) (CardAttachDistance :type "Float (double-precision)") (CardAttachHeight :type "Float (double-precision)"))
  (returns (CardSelf :type "/Game/GameBP/Blueprints/Gameplay/Actors/BP_Card Object Reference"))
  (set `self.CardAttachLoc` (`KismetMathLibrary.MakeVector` CardAttachDistance 0.0 CardAttachHeight))
  (`self.ConfigureAttachPoints`)
  (bind _output_get (set `self.CardData` CardData))
  (set `self.IndexInHand` IndexInHand)
  (`TextRenderComponent.K2_SetText` (`self.LabelText`) (`KismetTextLibrary.Conv_IntToText` (break `/Game/GameData/Data/Gameplay/ST_ClassicCard` _output_get)))
  (`TextRenderComponent.K2_SetText` (`self.LabelText1`) (`KismetTextLibrary.Conv_IntToText` (break `/Game/GameData/Data/Gameplay/ST_ClassicCard` _output_get)))
  (if (== (break `/Game/GameData/Data/Gameplay/ST_ClassicCard` _output_get) -1)
    (`ActorComponent.K2_DestroyComponent` (`self.CardCollisionTrigger`)))
  (return self))

(fn `Deselect`
  (`PrimitiveComponent.SetMaterial` (`self.CardMesh`) 0 "/Game/GameData/Materials/M_Card_Back.M_Card_Back") ; Change material
  (set `self.IsSelected` false))

(fn `Detach`
  (bind _rightjoinpoint (`self.RightJoinPoint`))
  (set `self.OrigAttachRotation` (`SceneComponent.K2_GetComponentRotation` _rightjoinpoint))
  (`SceneComponent.K2_DetachFromComponent` _rightjoinpoint "KeepWorld" "KeepWorld" "KeepWorld" true))

(fn `GetAttachPoint`
  (returns (AttachComponent :type "SceneComponent Object Reference"))
  (return (`self.RightJoinPoint`)))

(fn `GetPlayerController`
  (returns (PlayerControllerRef :type "/Game/GameBP/Blueprints/Gameplay/PC_Classic Object Reference"))
  (`/Engine/EditorBlueprintResources/StandardMacros.IsValid` (`self.PlayerControllerRef`)
    (:`Is Valid`
      _)
    (:`Is Not Valid`
      (bind _aspc_classic (cast `/Game/GameBP/Blueprints/Gameplay/PC_Classic` (`GameplayStatics.GetPlayerController` 0)))
      (set `self.PlayerControllerRef` _aspc_classic)))
  (return (`self.PlayerControllerRef`)))

(fn `MoveInDirection`
  (params (Direction :type "ETouchSwipeDirection Enum" :default "None") (Distance :type "Float (double-precision)") (Height :type "Float (double-precision)"))
  (locals (Result :type "Vector Structure"))
  (switch `ETouchSwipeDirection` Direction
    (:`Left`
      (set `local.Result` (`KismetMathLibrary.MakeVector` (* -1 Distance) 0.0 Height)))
    (:`Right`
      (set `local.Result` (`KismetMathLibrary.MakeVector` Distance 0.0 (* -1 Height)))))
  (`SceneComponent.K2_AddRelativeLocation` (`self.DummyRoot`) (`local.Result`) false false) ; TODO: Should interpolate
)

(fn `Reset Joins Attachment`
  (`SceneComponent.K2_SetWorldTransform` (`self.RightJoinPoint`) (`KismetMathLibrary.MakeTransform` (`SceneComponent.K2_GetComponentLocation` (`self.CardMesh`)) (`self.OrigAttachRotation`)) false false)
  (`self.ConfigureAttachPoints`))

(fn `Reset Root Attachment`
  (`SceneComponent.K2_AttachToComponent` (`self.CardMesh`) (`self.DummyRoot`) "None" "SnapToTarget" "SnapToTarget" "KeepWorld" true))

(fn `Seek in Direction`
  (params (Direction :type "ETouchSwipeDirection Enum" :default "None") (Amount :type "Float (double-precision)"))
  (locals (Result :type "Vector Structure" :default (0.0 0.0 0.0)))
  (bind _result (`local.Result`))
  (bind _cardcollisiontrigger (`self.CardCollisionTrigger`))
  (bind _cardcollisiontrigger_2 (`self.CardCollisionTrigger`))
  (bind (_boxextent_x _boxextent_y _boxextent_z) (`KismetMathLibrary.BreakVector` (`BoxComponent.BoxExtent` _cardcollisiontrigger)))
  (bind (_boxextent_x_2 _boxextent_y_2 _boxextent_z_2) (`KismetMathLibrary.BreakVector` (`BoxComponent.BoxExtent` _cardcollisiontrigger_2)))
  (switch `ETouchSwipeDirection` Direction
    (:`Left`
      (set `local.Result` (`KismetMathLibrary.MakeVector` (* -1 Amount)))
      (`BoxComponent.SetBoxExtent` _cardcollisiontrigger (`KismetMathLibrary.MakeVector` (/ _boxextent_x 2.0) _boxextent_y _boxextent_z) true))
    (:`Right`
      (set `local.Result` (`KismetMathLibrary.MakeVector` Amount))
      (`BoxComponent.SetBoxExtent` _cardcollisiontrigger_2 (`KismetMathLibrary.MakeVector` (* 2 _boxextent_x_2) _boxextent_y_2 _boxextent_z_2) true)))
  (`SceneComponent.K2_AddRelativeLocation` (`self.DummyRoot`) _result false false) ; TODO: Should interpolate
  (`SceneComponent.K2_AddRelativeLocation` (`self.CardCollisionTrigger`) (`KismetMathLibrary.MakeVector` (/ (.x _result) -2.0)) false false))

(fn `Select`
  (`PrimitiveComponent.SetMaterial` (`self.CardMesh`) 0 "/Game/GameData/Materials/OrangeMaterial.OrangeMaterial") ; Change material
  (set `self.IsSelected` true))

(fn `TogglePickupMode`
  (params (Activate :type Boolean))
  (if Activate
    (`PrimitiveComponent.SetSimulatePhysics` (`self.CardMesh`) true)
    (`self.Detach`)
    (set `self.IsPickedUp` true)
    (else
      (`PrimitiveComponent.SetSimulatePhysics` (`self.CardMesh`) false)
      (`self.Reset Joins Attachment`) ; Detach above, breaks the attach points loc
      (set `self.IsPickedUp` false))))

(fn `UserConstructionScript`)