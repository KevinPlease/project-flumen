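; Multiplayer game mode for the Classic card game, running the server side from player login through pair culling to the turn-based Roundtable.
; It tracks controllers and ready flags by player index, deals decks once all connect and starts Roundtable with the first player to finish culling.
; It relays culls and picks between controllers, masking picked cards with dummy data, while GameState handles phases, turns and finished players.
; The server shuts down when the last player leaves.
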(event `self.K2_PostLogin`
  (params (NewPlayer :type "PlayerController Object Reference"))
  ;[1 1 1] On LOGIN / LOGOUT -> Entry point of client connection
  (bind _playerindex (`self.AddPlayerInQueue`))
  (`/Game/GameBP/Blueprints/Gameplay/Base/PC_Classic_Base.Event Matched` (`self.GetPlayerByIndex` _playerindex) _playerindex))

(event `self.K2_OnLogout`
  (params (ExitingController :type "Controller Object Reference"))
  ;[1 1 1] On LOGIN / LOGOUT -> Entry point of client connection
  ;;[1 1 1] Player is disconnected
  (bind _aspc_classic_base (cast `/Game/GameBP/Blueprints/Gameplay/Base/PC_Classic_Base` ExitingController))
  (`self.UpdatePlayerDisconnected` _aspc_classic_base)
  (if (== (`BlueprintMapLibrary.Map_Length` (`self.PlayersReady`)) 0)
    (`GameServerManager.ShutdownServer` false)))

(event `self.Event Matched Player`
  (params (DesiredMatchSize :type Integer) (PlayerIndex :type Integer) (PlayerServerInfo :type "/Game/GameData/Data/Player/ST_PlayerServerInfo Structure"))
  ;[1 1 1] Player has joined server -> let client know that it is queued
  (if (== PlayerIndex 0)
    (set `self.PlayerCount` DesiredMatchSize))
  (`self.UpdatePlayerConnected` PlayerIndex PlayerServerInfo_PlayerName_4_82062F2C46B696FF488639B7BB118ADD)
  (if (`self.AreAllPlayersConnected`)
    (`self.Event All Players Connected`)
    (else
      (`KismetSystemLibrary.PrintString` "Not enough players connected"))))

(event `self.Event All Players Connected`
  ;[1 1 1] Player has joined server -> let client know that it is queued
  (`parent.Event All Players Connected`)
  (`KismetSystemLibrary.Delay` 1.0)
  (for _index (range (`self.PlayerCount`))
    (`/Game/GameBP/Blueprints/Gameplay/Base/PC_Classic_Base.Event Connected` (`self.GetPlayerByIndex` _index) (`/Game/GameBP/Blueprints/Gameplay/Objects/O_CardMaster.GetDecksForPlayer` (`self.CardMaster`) _index (`/Game/GameBP/Blueprints/Gameplay/GS_Classic.PlayerNames` (`self.GameStateRef`))))))

(event `self.Event Player Ready`
  (params (PlayerIndex :type Integer))
  (bind _gamestateref (`self.GameStateRef`))
  (bind (_gamerule_id _gamerule_playercount _gamerule_cardrepetition _gamerule_timeperturn) (break `/Game/GameData/Data/Gameplay/ST_GameRule` (`self.GameRule`)))
  ;[1 1 1] BEGIN gameplay once all players are ready i.e: decks created etc.
  (`self.SetPlayerReady` PlayerIndex)
  (if (`self.ArePlayersReady`)
    (for _index (range (`self.PlayerCount`))
      (`self.ResetPlayerReady` _index)
      (`/Game/GameBP/Blueprints/Gameplay/GS_Classic.Event Update Player Name` _gamestateref (`/Game/GameBP/Blueprints/Gameplay/GS_Classic.PlayerNames` _gamestateref)))
    (`/Game/GameBP/Blueprints/Gameplay/GS_Classic.Event Begin Culling` (`self.GameStateRef`) _gamerule_timeperturn)))

(event `self.Event Player Culled Cards`
  (params (PlayerIndex :type Integer) (SelectedPair :type "/Game/GameData/Data/Gameplay/ST_Selection_CardPair Structure"))
  (bind (_gamefinished _playerlost) (`self.CheckVictoryConditions`))
  (`parent.Event Player Culled Cards` PlayerIndex SelectedPair)
  (for _index (range (`self.PlayerCount`))
    (if (!= _index PlayerIndex)
      (`/Game/GameBP/Blueprints/Gameplay/Base/PC_Classic_Base.Event Other Player Culled` (`self.GetPlayerByIndex` _index) PlayerIndex SelectedPair)))
  (`|ExecutionSequence`
    (:`then_0`
      (switch `/Game/GameData/Data/Enums/E_GamePhases` (`/Game/GameBP/Blueprints/Gameplay/GS_Classic.GamePhase` (`self.GameStateRef`))
        (:`NewEnumerator0`
          ;[1 1 1] Check for remaining pairs -- if all players finished, tell GS to end the Culling phase
          (if (not (`/Game/GameBP/Blueprints/Gameplay/Objects/O_CardMaster.Has Remaining Pairs For Player` (`self.CardMaster`) PlayerIndex))
            (`self.SetPlayerReady` PlayerIndex)
            (if (`self.ArePlayersReady`)
              (`/Game/GameBP/Blueprints/Gameplay/GS_Classic.Event Begin RoundTable` (`self.GameStateRef`) (`self.FirstPlayerReady`) (`self.PlayerCount`)))))
        (:`NewEnumerator1`
          ;[1 1 1] Check if player who culled has remaining cards in hand
          (if (not (`/Game/GameBP/Blueprints/Gameplay/Objects/O_CardMaster.Has Remaining Cards For Player` (`self.CardMaster`) PlayerIndex)) :!label _label
            (`/Game/GameBP/Blueprints/Gameplay/GS_Classic.Event Player Finished` (`self.GameStateRef`) PlayerIndex false false 0.0))
          ;[1 1 1] Check for Finished Game
          (if _gamefinished
            (`/Game/GameBP/Blueprints/Gameplay/GS_Classic.Event Player Finished` (`self.GameStateRef`) _playerlost true false 0.0)))
        (:`NewEnumerator2`
          (goto _label))))
    (:`then_1`
      ;[1 1 1] Tell PC that cull is confirmed and finished server-side
      (`/Game/GameBP/Blueprints/Gameplay/Base/PC_Classic_Base.Event Cards Culled` (`self.GetPlayerByIndex` PlayerIndex) true SelectedPair))))

(event `self.Event Player Picked Card`
  (params (CardIndex :type Integer))
  (bind (_gamerule_id _gamerule_playercount _gamerule_cardrepetition _gamerule_timeperturn) (break `/Game/GameData/Data/Gameplay/ST_GameRule` (`self.GameRule`)))
  (bind _gamestateref (`self.GameStateRef`))
  (bind _gamestateref_2 (`self.GameStateRef`))
  (bind _activeplayerindex (`/Game/GameBP/Blueprints/Gameplay/GS_Classic.ActivePlayerIndex` _gamestateref))
  (bind _nextplayerindex (`/Game/GameBP/Blueprints/Gameplay/GS_Classic.NextPlayerIndex` _gamestateref))
  (bind _nextplayerindex_2 (`/Game/GameBP/Blueprints/Gameplay/GS_Classic.NextPlayerIndex` _gamestateref_2))
  (bind _nextplayerindex_3 (`/Game/GameBP/Blueprints/Gameplay/GS_Classic.NextPlayerIndex` (`self.GameStateRef`)))
  ;[1 1 1] Player picked a card from the next player -- End turn
  (`parent.Event Player Picked Card` CardIndex)
  (`/Game/GameBP/Blueprints/Gameplay/Base/PC_Classic_Base.Event Card Removed` (`self.GetPlayerByIndex` _nextplayerindex_3) CardIndex)
  (`/Game/GameBP/Blueprints/Gameplay/Objects/O_CardMaster.RemoveCardForPlayer` (`self.CardMaster`) _nextplayerindex_3 CardIndex)
  (for _index (range (`self.PlayerCount`))
    (`|ExecutionSequence`
      (:`then_0`
        (if (!= _index _activeplayerindex)
          (bind _pcontroller (`self.GetPlayerByIndex` _index))
          (`/Game/GameBP/Blueprints/Gameplay/Base/PC_Classic_Base.Event Other PC Added Card` _pcontroller (make `/Game/GameData/Data/Gameplay/ST_AddedCard` _activeplayerindex (make `/Game/GameData/Data/Gameplay/ST_ClassicCard` -1)))))
      (:`then_1`
        (if (!= _index _nextplayerindex)
          (`/Game/GameBP/Blueprints/Gameplay/Base/PC_Classic_Base.Event Other PC Removed Card` _pcontroller (make `/Game/GameData/Data/Gameplay/ST_RemovedCard` _nextplayerindex CardIndex))))))
  ;[1 1 1] Check if the BeingPicked player has remaining cards in hand -- Next Turn
  (if (`/Game/GameBP/Blueprints/Gameplay/Objects/O_CardMaster.Has Remaining Cards For Player` (`self.CardMaster`) _nextplayerindex_2)
    (`/Game/GameBP/Blueprints/Gameplay/GS_Classic.Event Next Turn` _gamestateref_2 (`KismetMathLibrary.Conv_IntToDouble` _gamerule_timeperturn))
    (else
      (`/Game/GameBP/Blueprints/Gameplay/GS_Classic.Event Player Finished` _gamestateref_2 _nextplayerindex_2 false true (`KismetMathLibrary.Conv_IntToDouble` _gamerule_timeperturn)))))

(fn `AddPlayerInQueue`
  (returns (PlayerIndex :type Integer))
  (locals (CurPlayerIndex :type Integer))
  (bind _curplayerindex (`local.CurPlayerIndex`))
  (bind _playersready (`self.PlayersReady`))
  (bind _output_get (set `local.CurPlayerIndex` (`BlueprintMapLibrary.Map_Length` _playersready)))
  (`BlueprintMapLibrary.Map_Add` _playersready _output_get)
  (bind _aspc_classic_base (cast `/Game/GameBP/Blueprints/Gameplay/Base/PC_Classic_Base` (`GameplayStatics.GetPlayerController` _curplayerindex)))
  (`BlueprintMapLibrary.Map_Add` (`self.ConnectedPlayers`) _curplayerindex _aspc_classic_base)
  (return _curplayerindex))

(fn `AreAllPlayersConnected`
  (returns (ReturnValue :type Boolean))
  (return (== (`BlueprintMapLibrary.Map_Length` (`self.PlayersReady`)) (`self.PlayerCount`))))

(fn `ArePlayersReady`
  (returns (AreReady :type Boolean))
  (bind _values (`BlueprintMapLibrary.Map_Values` (`self.PlayersReady`)))
  (return (not (`KismetArrayLibrary.Array_Contains` _values))))

(fn `GetPlayerByIndex`
  (params (PlayerIndex :type Integer))
  (returns (PController :type "/Game/GameBP/Blueprints/Gameplay/Base/PC_Classic_Base Object Reference"))
  (return (`BlueprintMapLibrary.Map_Find` (`self.ConnectedPlayers`) PlayerIndex)))

(fn `RemovePlayerFromQueue`
  (params (Index :type Integer))
  (`BlueprintMapLibrary.Map_Remove` (`self.PlayersReady`) Index)
  (`BlueprintMapLibrary.Map_Remove` (`self.ConnectedPlayers`) Index)
  (return))

(fn `ResetPlayerReady`
  (params (PlayerIndex :type Integer))
  (`BlueprintMapLibrary.Map_Add` (`self.PlayersReady`) PlayerIndex))

(fn `SetPlayerReady`
  (params (PlayerIndex :type Integer))
  (bind _values (`BlueprintMapLibrary.Map_Values` (`self.PlayersReady`)))
  (if (not (`KismetArrayLibrary.Array_Contains` _values true))
    (set `self.FirstPlayerReady` PlayerIndex))
  (`BlueprintMapLibrary.Map_Add` (`self.PlayersReady`) PlayerIndex true))

(fn `UpdatePlayerConnected`
  (params (PlayerIndex :type Integer) (PlayerName :type String))
  (`KismetArrayLibrary.Array_Set` (`/Game/GameBP/Blueprints/Gameplay/GS_Classic.PlayerNames` (`self.GameStateRef`)) PlayerIndex PlayerName true))

(fn `UpdatePlayerDisconnected`
  (params (PlayerController :type "/Game/GameBP/Blueprints/Gameplay/Base/PC_Classic_Base Object Reference"))
  (locals (FoundPlayerIndex :type Integer))
  (bind _connectedplayers (`self.ConnectedPlayers`))
  (bind _keys (`BlueprintMapLibrary.Map_Keys` _connectedplayers))
  (for _array_element _keys
    (if (== (`BlueprintMapLibrary.Map_Find` _connectedplayers _array_element) PlayerController)
      (set `local.FoundPlayerIndex` _array_element)
      (break)))
  (`self.RemovePlayerFromQueue` (`local.FoundPlayerIndex`)))

(fn `UserConstructionScript`
  (`parent.UserConstructionScript`))