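; Player controller for the Classic mode of a multiplayer card game with pair culling and turn-based picking from other players' hands.
; Matchmaking, readiness and card actions go to GM_Classic through server events, while GS_Classic dispatchers drive the local phase, HUD and camera seat moves.
; It spawns a board rotated to the player's seat.
; Touch input separates taps for selection from long-press drags that shift and reorder cards.
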(event `Event Matched`
  (params (PlayerIndex :type Integer))
  ;[1 1 1] Initial begin for PC --- Set index -> Send desired match size to GM
  (set `self.PlayerIndex` PlayerIndex)
  (bind _asgi_core (cast `/Game/GameBP/Blueprints/GI_Core` (`GameplayStatics.GetGameInstance`)))
  (bind _output_get (set `self.GameInstRef` _asgi_core))
  (`self.ToServer: Matched` (`/Game/GameBP/Blueprints/GI_Core.Matchmaking Size` _output_get) (`self.PlayerIndex`)))

(event `ToServer: Matched`
  (params (DesiredMatchSize :type Integer) (PlayerIndex :type Integer))
  ;[1 1 1] Initial begin for PC --- Set index -> Send desired match size to GM
  (bind _asgm_classic (cast `/Game/GameBP/Blueprints/Gameplay/GM_Classic` (`GameplayStatics.GetGameMode`)))
  (bind _output_get (set `self.SV_GameModeRef` _asgm_classic))
  (`/Game/GameBP/Blueprints/Gameplay/GM_Classic.Event Matched Player` _output_get DesiredMatchSize))

(event `Event Connected`
  (params (DeckData :type "Array of /Game/GameData/Data/Gameplay/Wrappers/ST_CardList Structure (by ref)"))
  (bind _gamestateref (`self.GameStateRef`))
  ;[1 1 1] Player connected with other player/s -- create HUD ...
  (bind _asc_classic (cast `/Game/GameBP/Blueprints/Gameplay/C_Classic` (`GameplayStatics.GetPlayerCharacter` 0)))
  (set `self.CharacterRef` _asc_classic)
  (bind _returnvalue (`|CreateWidget` "/Game/GameBP/Blueprints/Gameplay/UI/WB_HUD.WB_HUD_C" self))
  (bind _output_get (set `self.WB_HUD` _returnvalue))
  (`UserWidget.AddToViewport` _output_get 0)
  (bind _decks (`self.CreateDeckObj` DeckData))
  (`self.Create Board` _decks)
  (bind _asgs_classic (cast `/Game/GameBP/Blueprints/Gameplay/GS_Classic` (`GameplayStatics.GetGameState`)))
  (set `self.GameStateRef` _asgs_classic)
  (`|ExecutionSequence`
    (:`then_0`
      (add `/Game/GameBP/Blueprints/Gameplay/GS_Classic.DispatchBeginCulling` _gamestateref (`|CreateDelegate` :!event `Event On Begin Culling`))
      (add `/Game/GameBP/Blueprints/Gameplay/GS_Classic.DispatchEndCulling` _gamestateref (`|CreateDelegate` :!event `Event Finished Culling`))
      (add `/Game/GameBP/Blueprints/Gameplay/GS_Classic.DispatchNextTurn` _gamestateref (`|CreateDelegate` :!event `Event On Next Turn`))
      (add `/Game/GameBP/Blueprints/Gameplay/GS_Classic.DispatchTransitionPhase` _gamestateref (`|CreateDelegate` :!event `Event On Transition Phase`))
      (add `/Game/GameBP/Blueprints/Gameplay/GS_Classic.DispatchEmptyDeckForPlayer` _gamestateref (`|CreateDelegate` :!event `Event On Empty Deck`))
      (add `/Game/GameBP/Blueprints/Gameplay/GS_Classic.DispatchGameOver` _gamestateref (`|CreateDelegate` :!event `Event Game Over`)))
    (:`then_1`
      ;[1 1 1] Player has connected successfully and is ready to start game
      (`WidgetBlueprintLibrary.SetInputMode_GameAndUIEx` self null "DoNotLock" false)
      (`self.To Server: Ready To Play` (`self.PlayerIndex`)) ; Player setup finished
    )))

(event `To Server: Ready To Play`
  (params (PlayerIndex :type Integer))
  ;[1 1 1] Player has connected successfully and is ready to start game
  (bind _asgm_classic (cast `/Game/GameBP/Blueprints/Gameplay/GM_Classic` (`GameplayStatics.GetGameMode`)))
  (bind _output_get (set `self.SV_GameModeRef` _asgm_classic))
  (`/Game/GameBP/Blueprints/Gameplay/GM_Classic.Event Player Ready` _output_get PlayerIndex))

(event `Event Clicked Card`
  (params (ClickedCardActor :type "/Game/GameBP/Blueprints/Gameplay/Actors/BP_Card Object Reference"))
  (bind _firstselectedcardlabel (`self.FirstSelectedCardLabel`))
  (bind _indexinhand (`/Game/GameBP/Blueprints/Gameplay/Actors/BP_Card.IndexInHand` ClickedCardActor))
  (bind _carddata_label (break `/Game/GameData/Data/Gameplay/ST_ClassicCard` (`/Game/GameBP/Blueprints/Gameplay/Actors/BP_Card.CardData` ClickedCardActor)))
  ;[1 1 1] Input: Single Click on Card
  (if (not (`/Game/GameBP/Blueprints/Gameplay/Actors/BP_Card.IsSelected` ClickedCardActor))
    (`/Game/GameBP/Blueprints/Gameplay/Actors/BP_Card.Select` ClickedCardActor)
    (switch `/Game/GameData/Data/Enums/E_PlayerPhases` (`self.ActivePhase`)
      (:`NewEnumerator4`
        (`/Engine/EditorBlueprintResources/StandardMacros.CompareInt` _firstselectedcardlabel -1 :!label _label ; Check if 2 cards have been selected
          (:`>`
            (set `self.SecondCardIndex` _indexinhand)
            (`self.To Server: Culled Cards` (`self.PlayerIndex`) (make `/Game/GameData/Data/Gameplay/ST_Selection_CardPair` _firstselectedcardlabel _carddata_label (`self.FirstCardIndex`) (`self.SecondCardIndex`)))
            (`self.ResetSelection`))
          (:`==`
            (set `self.FirstSelectedCardLabel` _carddata_label)
            (set `self.FirstCardIndex` _indexinhand))))
      (:`NewEnumerator0`
        (goto _label))
      (:`NewEnumerator1`
        (`self.To Server: Picked Card From Player` _indexinhand))
      (:`NewEnumerator6`
        (goto _label)))
    (else
      (`/Game/GameBP/Blueprints/Gameplay/Actors/BP_Card.Deselect` ClickedCardActor)
      (`self.ResetSelection`))))

(event `Event Player Forfeits`
  ;[1 1 1] Player forfeits
  (`/Game/GameBP/Blueprints/GI_Core.LoadClientMap` (`self.GameInstRef`)))

(event `self.ReceiveTick`
  (params (DeltaSeconds :type "Float (single-precision)"))
  ;[1 1 1] Handle touch input
  (if (`self.IsHoldingCard`)
    (`self.UpdateHoldingCard`)))

(event `InputTouch`
  (params (Location :type "Vector Structure") (FingerIndex :type "ETouchIndex Enum"))
  ;[1 1 1] Handle touch input
  (:`Pressed`
    (bind _asbp_card (cast `/Game/GameBP/Blueprints/Gameplay/Actors/BP_Card` (`.HitActor` (`GameplayStatics.BreakHitResult` (`self.GetHitResultUnderFingerForObjects` "Touch1" (`|MakeArray` "ObjectTypeQuery1" :!type "EObjectTypeQuery Enum"))))))
    (`self.InputPress` :!label _label_2
      (:`LongPress`
        (if (not (`self.IsHoldingCard`))
          (`self.StartCardHolding` _asbp_card)))
      (:`SinglePress`
        (`self.IsValidSelection` _asbp_card
          (:`Valid`
            (`self.Event Clicked Card` _asbp_card))))))
  (:`Released`
    (`|ExecutionSequence`
      (:`then_0`
        (goto _label_2 :!via `Released`))
      (:`then_1`
        (if (`self.IsHoldingCard`) :!label _label_3
          (`self.StopCardHolding`)))))
  (:`Moved`
    (`/Engine/EditorBlueprintResources/StandardMacros.DoOnce` false :!label _label_4
      (:`Completed`
        (bind _asbp_card_2 (`self.CheckMovingInputBounds`)
          (:`Overlapped Seeking Card`
            (`self.Event Card Seeking Position` _asbp_card_2))
          (:`No Card But Within Deck Bounds`
            (`self.Event Reset Card Seeking` :!label _label_5)
            (goto _label_3))
          (:`Out Of Deck Bounds`
            (goto _label_5))
          (:`Default`
            (`self.InternalResetMovingInput`)))))))

(event `InternalResetMovingInput`
  ;[1 1 1] Handle touch input
  (goto _label_4 :!via `Reset`))

(event `Event Reset Card Seeking`
  ;[1 1 1] Handle touch input
  (`/Engine/EditorBlueprintResources/StandardMacros.IsValid` (`self.CurSeekingCard`)
    (:`Is Valid`
      (`/Game/GameBP/Blueprints/Gameplay/Actors/BP_CardDeck.Reset Card SeekingShifts` (`self.PlayerDeck`))
      (set `self.CurSeekingCard` null)
      (goto _label_4 :!via `Reset`))
    (:`Is Not Valid`
      (goto _label_4 :!via `Reset`))))

(event `Event Reset For Next Phase`
  (bind _asbp_card (`/Game/GameBP/Blueprints/Gameplay/Actors/BP_CardDeck.Get Card As Actor` (`self.PlayerDeck`) (`self.FirstCardIndex`)))
  ;[1 1 1] Reset all selections, card seeking
  (`self.Event Reset Card Seeking`)
  (if (`self.IsHoldingCard`)
    (`self.StopCardHolding`))
  (`/Engine/EditorBlueprintResources/StandardMacros.IsValid` _asbp_card
    (:`Is Valid`
      (if (`/Game/GameBP/Blueprints/Gameplay/Actors/BP_Card.IsSelected` _asbp_card)
        (`/Game/GameBP/Blueprints/Gameplay/Actors/BP_Card.Deselect` _asbp_card)
        (`self.ResetSelection`)))))

(event `Event On Transition Phase`
  ;[1 1 1] Next Turn
  (if (`self.IsInGameplay`)
    (set `self.ActivePhase` "NewEnumerator6")
    (`self.UI Update Player Phase`)
    (`/Game/GameBP/Blueprints/Gameplay/C_Classic.Event Back to Original Seat` (`self.CharacterRef`))))

(event `Event On Next Turn`
  (params (PlayerIndex :type Integer) (NextPlayerIndex :type Integer) (FirstTime :type Boolean))
  (bind _characterref (`self.CharacterRef`))
  ;[1 1 1] Next Turn
  (if (`self.IsInGameplay`)
    (if FirstTime
      (`self.UI Update Game Phase`))
    (`self.UpdatePhase` PlayerIndex NextPlayerIndex)
    (`self.UI Update Player Phase`)
    (if (`|EnumEquality` (`self.ActivePhase`) "NewEnumerator1")
      (`self.Event Reset For Next Phase`)
      (`/Game/GameBP/Blueprints/Gameplay/C_Classic.Event Move to Seat Transform` _characterref (`/Game/GameBP/Blueprints/Gameplay/Actors/BP_GameBoard.Get Seat Transform For Player` (`self.GameBoard`) NextPlayerIndex))
      (`self.UpdatePostAnimInput` true)
      (else
        (`/Game/GameBP/Blueprints/Gameplay/C_Classic.Event Back to Original Seat` _characterref)
        (`self.UpdatePostAnimInput` false)))))

(event `Event Card Seeking Position`
  (params (InCard :type "/Game/GameBP/Blueprints/Gameplay/Actors/BP_Card Object Reference"))
  ;[1 1 1] A picked up card is seeking for a new position -- Shift cards left/right to make room while Picked up card traverses Deck
  (`/Engine/EditorBlueprintResources/StandardMacros.IsValid` (`self.CurSeekingCard`) ; Check for previous shifted card to move back into place
    (:`Is Valid`
      (if (== (`self.CurSeekingCard`) InCard)
        (`self.InternalResetMovingInput` :!label _label)
        (else
          (`/Game/GameBP/Blueprints/Gameplay/Actors/BP_Card.Seek in Direction` (`self.CurSeekingCard`) "None")
          (if true :!label _label_2
            (bind _output_get (set `self.CurSeekingCard` InCard))
            (set `self.CurSeekingCardOriginalLoc` (`SceneComponent.K2_GetComponentLocation` (`/Game/GameBP/Blueprints/Gameplay/Actors/BP_Card.CardMesh` _output_get))) ; used in case card is confirmed for reposition, separate event
            (`/Game/GameBP/Blueprints/Gameplay/Actors/BP_CardDeck.ShiftCardsFrom` (`self.PlayerDeck`) (`/Game/GameBP/Blueprints/Gameplay/Actors/BP_Card.IndexInHand` _output_get) "Right")
            (goto _label)
            (else
              (`self.InternalResetMovingInput`))))))
    (:`Is Not Valid`
      (goto _label_2))))

(event `Event On Empty Deck`
  (params (PlayerIndex :type Integer))
  ;[1 1 1] Player emptied Deck -- go into spectating mode
  (if (== PlayerIndex (`self.PlayerIndex`))
    (set `self.ActivePhase` "NewEnumerator3")
    (`WidgetBlueprintLibrary.SetInputMode_UIOnlyEx` self null)
    (`self.UI Update Player Phase`)
    (`/Game/GameBP/Blueprints/Gameplay/C_Classic.Event Back to Original Seat` (`self.CharacterRef`))
    (else
      ;[1 0.5744 0.09237] TODO: Might update GameBoard to show something in the location of the player-who-'won''s deck
      (`KismetSystemLibrary.PrintString` "Hello"))))

(event `Event Card Removed`
  (params (CardIndex :type Integer))
  ;[1 1 1] Card was removed/added - notify own Deck
  (`/Game/GameBP/Blueprints/Gameplay/Actors/BP_CardDeck.Event Removed Card` (`self.PlayerDeck`) CardIndex)
  (`self.ResetSelection`) ; Case when 1 card was selected during culling process,\nbut other player picked it during his/her Picking phase
)

(event `Event Card Added`
  (params (CardData :type "/Game/GameData/Data/Gameplay/ST_ClassicCard Structure"))
  ;[1 1 1] Card was removed/added - notify own Deck
  (`/Game/GameBP/Blueprints/Gameplay/Actors/BP_CardDeck.Event Added Card` (`self.PlayerDeck`) CardData))

(event `ToServer: CardsRepositioned`
  (params (SubjectCardIndex :type Integer) (TargetCardIndex :type Integer))
  ;[1 1 1] Cards repositioned in deck -- notify GM to update indices
  (`/Game/GameBP/Blueprints/Gameplay/GM_Classic.Event Player Repositioned Cards` (`self.SV_GameModeRef`) (`self.PlayerIndex`) SubjectCardIndex TargetCardIndex))

(event `Event Other PC Removed Card`
  (params (RemovedCardDeal :type "/Game/GameData/Data/Gameplay/ST_RemovedCard Structure"))
  ;[1 1 1] Other PC made changes to his/her deck -- update actors
  (`/Game/GameBP/Blueprints/Gameplay/Actors/BP_GameBoard.Event Card Removed By Player` (`self.GameBoard`) RemovedCardDeal))

(event `Event Other PC Added Card`
  (params (ST_AddedCard :type "/Game/GameData/Data/Gameplay/ST_AddedCard Structure (by ref)"))
  ;[1 1 1] Other PC made changes to his/her deck -- update actors
  (`/Game/GameBP/Blueprints/Gameplay/Actors/BP_GameBoard.Event Card Added By Player` (`self.GameBoard`) ST_AddedCard))

(event `Event Game Over`
  (params (PlayerLost :type Integer))
  ;[1 1 1] A player has lost -- check if self -- Game Over
  (`|ExecutionSequence`
    (:`then_0`
      (if (== PlayerLost (`self.PlayerIndex`))
        (`WidgetBlueprintLibrary.SetInputMode_UIOnlyEx` self null)
        (`/Game/GameBP/Blueprints/Gameplay/C_Classic.Event Back to Original Seat` (`self.CharacterRef`))))
    (:`then_1`
      (`/Game/GameBP/Blueprints/Gameplay/UI/WB_HUD.ShowGameResults` (`self.WB_HUD`) (`/Game/GameBP/Blueprints/Gameplay/GS_Classic.GetGameResults` (`self.GameStateRef`)))
      (`self.UI Update Game Phase`))))

(event `To Server: Picked Card From Player`
  (params (PickedCardIndex :type Integer))
  ;[1 1 1] Tell GM about the picked card index
  (`/Game/GameBP/Blueprints/Gameplay/GM_Classic.Event Player Picked Card` (`self.SV_GameModeRef`) PickedCardIndex))

(event `Event Return to Main Menu`
  ;[1 1 1] A player has lost -- check if self -- Game Over
  (set `/Game/GameBP/Blueprints/GI_Core.GameResult` (`/Game/GameBP/Blueprints/Gameplay/GS_Classic.GetResultForPlayer` (`self.GameStateRef`) (`self.PlayerIndex`)) (`self.GameInstRef`))
  (`GameplayStatics.OpenLevel` (`self.ClientLevelName`)))

(event `Event On Begin Culling`
  ;[1 1 1] Begin Phase
  (set `self.ActivePhase` "NewEnumerator4")
  (`self.UI Update Game Phase`)
  (`self.UI Update Player Phase`))

(event `To Server: Culled Cards`
  (params (PlayerIndex :type Integer) (CardPair :type "/Game/GameData/Data/Gameplay/ST_Selection_CardPair Structure"))
  ;[1 1 1] Tell server cards of Culling attempt
  (`/Game/GameBP/Blueprints/Gameplay/GM_Classic.Event Player Culled Cards` (`self.SV_GameModeRef`) PlayerIndex CardPair))

(event `Event Cards Culled`
  (params (IsValid :type Boolean) (CardPair :type "/Game/GameData/Data/Gameplay/ST_Selection_CardPair Structure"))
  (bind (_firstlabel _secondlabel _firstposition _secondposition) (break `/Game/GameData/Data/Gameplay/ST_Selection_CardPair` CardPair))
  (bind _playerdeck (`self.PlayerDeck`))
  ;[1 1 1] Tell server cards of Culling attempt
  (if IsValid
    (`/Game/GameBP/Blueprints/Gameplay/Actors/BP_CardDeck.Event Cull Cards` _playerdeck (make `/Game/GameData/Data/Gameplay/ST_Selection_CardPair` 0 0 _firstposition _secondposition))
    (else
      (`/Game/GameBP/Blueprints/Gameplay/Actors/BP_CardDeck.Event Bad Cull Attempt` _playerdeck (make `/Game/GameData/Data/Gameplay/ST_Selection_CardPair` 0 0 _firstposition _secondposition)))))

(event `Event Other Player Culled`
  (params (OtherPlayerIndex :type Integer) (CardPair :type "/Game/GameData/Data/Gameplay/ST_Selection_CardPair Structure"))
  ;[1 1 1] Other player has culled cards -- update GameBoard
  (`/Game/GameBP/Blueprints/Gameplay/Actors/BP_GameBoard.Event Pair Removed By Player` (`self.GameBoard`) OtherPlayerIndex CardPair))

(event `Event Finished Culling`
  ;[1 1 1] Server says Culling phase is over - disable input etc...
  (`WidgetBlueprintLibrary.SetInputMode_UIOnlyEx` self null)
  (set `self.ActivePhase` "NewEnumerator0")
  (`self.UI Update Game Phase`)
  (`self.UI Update Player Phase`))

(fn `Create Board`
  (params (Decks :type "Array of /Game/GameBP/Blueprints/Gameplay/Objects/O_CardDeck Object Reference"))
  (bind _playerprofile (`/Game/GameBP/Blueprints/GI_Core.PlayerProfile` (`self.GameInstRef`)))
  (bind _returnvalue (`|SpawnActorFromClass` "/Game/GameBP/Blueprints/Gameplay/Actors/BP_GameBoard.BP_GameBoard_C" (`self.GetSpawnLocation`) "Undefined" "OverrideRootScale" self (`/Game/GameBP/Blueprints/Client/Objects/O_PlayerProfile.GetBoardTheme` _playerprofile) (`/Game/GameBP/Blueprints/Client/Objects/O_PlayerProfile.GetCardTheme` _playerprofile) null))
  (bind _output_get (set `self.GameBoard` _returnvalue))
  (`/Game/GameBP/Blueprints/Gameplay/Actors/BP_GameBoard.Event Create With Data` _output_get Decks (`self.PlayerIndex`))
  (set `self.PlayerDeck` (`/Game/GameBP/Blueprints/Gameplay/Actors/BP_GameBoard.GetDeckActorForPlayer` _output_get (`self.PlayerIndex`))))

(fn `CreateDeckObj`
  (params (DeckData :type "Array of /Game/GameData/Data/Gameplay/Wrappers/ST_CardList Structure"))
  (returns (Decks :type "Array of /Game/GameBP/Blueprints/Gameplay/Objects/O_CardDeck Object Reference"))
  (locals (CurCardDeck :type "/Game/GameBP/Blueprints/Gameplay/Objects/O_CardDeck Object Reference") (DeckObjs :type "Array of /Game/GameBP/Blueprints/Gameplay/Objects/O_CardDeck Object Reference"))
  (bind _curcarddeck (`local.CurCardDeck`))
  (for (_array_element _array_index) DeckData
    (if (== _array_index (`self.PlayerIndex`))
      (bind _returnvalue (`|GenericCreateObject` "/Game/GameBP/Blueprints/Gameplay/Objects/O_PlayerDeck.O_PlayerDeck_C" self))
      (set `local.CurCardDeck` _returnvalue)
      (else
        (bind _returnvalue_2 (`|GenericCreateObject` "/Game/GameBP/Blueprints/Gameplay/Objects/O_EnemyDeck.O_EnemyDeck_C" self))
        (set `local.CurCardDeck` _returnvalue_2)))
    (`/Game/GameBP/Blueprints/Gameplay/Objects/O_CardDeck.Create` _curcarddeck (`.Cards_3_284AFC5841CB3129500CB1B12D8401DE` (break `/Game/GameData/Data/Gameplay/Wrappers/ST_CardList` _array_element)))
    (`KismetArrayLibrary.Array_Add` (`local.DeckObjs`) _curcarddeck))
  (return (`local.DeckObjs`)))

(fn `GetSpawnLocation`
  (returns (SpawnTransform :type "Transform Structure"))
  (locals (YawMultiplier :type "Float (double-precision)" :default 0.0))
  (switch `int` (`self.PlayerIndex`)
    (:`0`
      (set `local.YawMultiplier` 0.0))
    (:`1`
      (set `local.YawMultiplier` 90.0))
    (:`2`
      (set `local.YawMultiplier` -90.0))
    (:`3`
      (set `local.YawMultiplier` -180.0)))
  (return (`KismetMathLibrary.MakeTransform` (0.0 0.0 0.0) (`KismetMathLibrary.MakeRotator` 0.0 0.0 (`local.YawMultiplier`)))))

(fn `IsHoldingCard`
  (returns (IsHolding :type Boolean))
  (return (`KismetSystemLibrary.IsValid` (`self.HoldingCard`))))

(fn `IsInGameplay`
  (returns (InGameplay :type Boolean))
  (return (`|EnumInequality` (`self.ActivePhase`) "NewEnumerator3")))

(fn `IsValidSeekingCardPos`
  (params (Card :type "/Game/GameBP/Blueprints/Gameplay/Actors/BP_Card Object Reference"))
  (returns (ReturnValue :type Boolean))
  (bind _holdingcard (`self.HoldingCard`))
  (if (`KismetSystemLibrary.IsValid` _holdingcard)
    (return (!= (`/Game/GameBP/Blueprints/Gameplay/Actors/BP_Card.IndexInHand` Card) (+ (`/Game/GameBP/Blueprints/Gameplay/Actors/BP_Card.IndexInHand` _holdingcard) 1)))
    (else
      (return false))))

(fn `ResetSelection`
  (set `self.FirstSelectedCardLabel` -1)
  (set `self.FirstCardIndex` -1)
  (set `self.SecondCardIndex` -1))

(fn `StartCardHolding`
  (params (CardActor :type "/Game/GameBP/Blueprints/Gameplay/Actors/BP_Card Object Reference"))
  (bind _cardhandler (`self.CardHandler`))
  (bind _cardmesh (`/Game/GameBP/Blueprints/Gameplay/Actors/BP_Card.CardMesh` CardActor))
  (set `self.PickupCardOrigLoc` (`SceneComponent.K2_GetComponentLocation` _cardmesh))
  (`/Game/GameBP/Blueprints/Gameplay/Actors/BP_Card.TogglePickupMode` CardActor true)
  (`PhysicsHandleComponent.GrabComponentAtLocation` _cardhandler _cardmesh "None" (`self.PickupCardOrigLoc`))
  (set `self.HoldingCardComponent` (`PhysicsHandleComponent.GetGrabbedComponent` _cardhandler))
  (set `self.HoldingCard` CardActor))

(fn `StopCardHolding`
  (bind _curseekingcard (`self.CurSeekingCard`))
  (bind _indexinhand (`/Game/GameBP/Blueprints/Gameplay/Actors/BP_Card.IndexInHand` (`self.CurSeekingCard`)))
  (bind _indexinhand_2 (`/Game/GameBP/Blueprints/Gameplay/Actors/BP_Card.IndexInHand` (`self.HoldingCard`)))
  (`PhysicsHandleComponent.ReleaseComponent` (`self.CardHandler`))
  (`/Game/GameBP/Blueprints/Gameplay/Actors/BP_Card.TogglePickupMode` (`self.HoldingCard`) false)
  (if (`KismetSystemLibrary.IsValid` _curseekingcard)
    (if (`self.IsValidSeekingCardPos` _curseekingcard)
      (set `self.HoldingCardComponent` null)
      (`/Game/GameBP/Blueprints/Gameplay/Actors/BP_CardDeck.Event Reposition Cards` (`self.PlayerDeck`) _indexinhand_2 _indexinhand)
      (`self.ToServer: CardsRepositioned` _indexinhand_2 _indexinhand)
      (set `self.HoldingCard` null)
      (set `self.CurSeekingCard` null)
      (else
        ;[1 1 1] Invalid pos -- reset card pos back to its original starting pos
        (`SceneComponent.K2_SetWorldLocation` (`self.HoldingCardComponent`) (`self.PickupCardOrigLoc`) false false :!label _label)
        (set `self.HoldingCardComponent` null)
        (set `self.HoldingCard` null)
        (set `self.CurSeekingCard` null)
        (`/Game/GameBP/Blueprints/Gameplay/Actors/BP_CardDeck.Reset Card SeekingShifts` (`self.PlayerDeck`))))
    (else
      (goto _label))))

(fn `UI Update Game Phase`
  (bind _wb_hud (`self.WB_HUD`))
  (bind _gamephase (`/Game/GameBP/Blueprints/Gameplay/GS_Classic.GamePhase` (`self.GameStateRef`)))
  (switch `/Game/GameData/Data/Enums/E_GamePhases` _gamephase
    (:`NewEnumerator0`
      (`/Game/GameBP/Blueprints/Gameplay/UI/WB_HUD.SetGamePhaseText` _wb_hud _gamephase))
    (:`NewEnumerator1`
      (`/Game/GameBP/Blueprints/Gameplay/UI/WB_HUD.ToggleGamePhaseText` _wb_hud false :!label _label))
    (:`NewEnumerator2`
      (goto _label))
    (:`NewEnumerator3`
      (goto _label))))

(fn `UI Update Phase Counter`
  (params (Counter :type Integer))
  (`/Game/GameBP/Blueprints/Gameplay/UI/WB_HUD.SetCounter` (`self.WB_HUD`) Counter))

(fn `UI Update Player Phase`
  (`/Game/GameBP/Blueprints/Gameplay/UI/WB_HUD.SetPlayerPhaseText` (`self.WB_HUD`) (`self.PlayerIndex`) (`self.ActivePhase`)))

(fn `UpdateHoldingCard`
  (bind (_pickupcardorigloc_x _pickupcardorigloc_y _pickupcardorigloc_z) (`KismetMathLibrary.BreakVector` (`self.PickupCardOrigLoc`)))
  (switch `/Game/GameData/Data/Enums/E_Axis` (`/Game/GameBP/Blueprints/Gameplay/Actors/BP_GameBoard.GetHorizontalAxisForPlayer` (`self.GameBoard`) (`self.PlayerIndex`))
    (:`NewEnumerator0`
      (`SceneComponent.K2_SetWorldLocation` (`self.HoldingCardComponent`) (`KismetMathLibrary.MakeVector` (.x (`.Location` (`GameplayStatics.BreakHitResult` (`self.GetHitResultUnderFingerForObjects` "Touch1" (`|MakeArray` "ObjectTypeQuery2" :!type "EObjectTypeQuery Enum"))))) _pickupcardorigloc_y _pickupcardorigloc_z) false false))
    (:`NewEnumerator1`
      (`SceneComponent.K2_SetWorldLocation` (`self.HoldingCardComponent`) (`KismetMathLibrary.MakeVector` _pickupcardorigloc_x (.y (`.Location` (`GameplayStatics.BreakHitResult` (`self.GetHitResultUnderFingerForObjects` "Touch1" (`|MakeArray` "ObjectTypeQuery2" :!type "EObjectTypeQuery Enum"))))) _pickupcardorigloc_z) false false))))

(fn `UpdatePhase`
  (params (ActivePlayerIndex :type Integer) (NextPlayerIndex :type Integer))
  (bind _playerindex (`self.PlayerIndex`))
  (if (== ActivePlayerIndex _playerindex)
    (if (`/Game/GameBP/Blueprints/Gameplay/GS_Classic.IsLastPlayer` (`self.GameStateRef`) (`self.PlayerIndex`))
      (set `self.ActivePhase` "NewEnumerator0")
      (else
        (set `self.ActivePhase` "NewEnumerator1")))
    (elif (== NextPlayerIndex _playerindex)
      (set `self.ActivePhase` "NewEnumerator2")
      (else
        (set `self.ActivePhase` "NewEnumerator0")))))

(fn `UserConstructionScript`)