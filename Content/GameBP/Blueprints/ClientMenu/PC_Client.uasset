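; Player controller for the client menu, which creates the main menu widget and acts as the bridge to its UI.
; On BeginPlay it caches the GI_Core game instance, loads options, then shows the menu with the player profile's display name and coins.
; It also exposes functions to show game rewards and toggle the loading screen.
; Coin changes animate through a timeline that lerps the player bar counter toward the profile total.
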(event `Event Update Player Coins`
  ;[1 1 1] Animate coins update for Player status bar
  (set `self.CurBeforeCoins` (`KismetMathLibrary.Conv_IntToDouble` (`/Game/GameBP/Blueprints/ClientMenu/UI/WB_Player.Coins` (`/Game/GameBP/Blueprints/ClientMenu/UI/WB_MainMenu.WB_PlayerBar` (`self.WB_MainMenu`)))))
  (set `self.CurTotalCoins` (`KismetMathLibrary.Conv_IntToDouble` (`/Game/GameBP/Blueprints/ClientMenu/Objects/O_PlayerProfile.GetCoins` (`/Game/GameBP/Blueprints/GI_Core.PlayerProfile` (`self.GameInstRef`)))))
  (bind (_direction _animationtime) (`Timeline|TimelineAnimateCoinUpdate` :!via `PlayFromStart`)
    (:`Update`
      (set `/Game/GameBP/Blueprints/ClientMenu/UI/WB_Player.Coins` (`KismetMathLibrary.FTrunc` (`KismetMathLibrary.Lerp` (`self.CurBeforeCoins`) (`self.CurTotalCoins`) _animationtime)) (`/Game/GameBP/Blueprints/ClientMenu/UI/WB_MainMenu.WB_PlayerBar` (`self.WB_MainMenu`))))))

(event `self.ReceiveBeginPlay`
  ;[1 1 1] Begin Play
  (bind _asgi_core (cast `/Game/GameBP/Blueprints/GI_Core` (`GameplayStatics.GetGameInstance`)))
  (bind _output_get (set `self.GameInstRef` _asgi_core))
  (`/Game/GameBP/Blueprints/GI_Core.LoadOptions` _output_get)
  (`self.Event Show Main Menu`))

(event `Event Show Main Menu`
  ;[1 1 1] Create and show Main Menu
  (bind _returnvalue (`|CreateWidget` "/Game/GameBP/Blueprints/ClientMenu/UI/WB_MainMenu.WB_MainMenu_C" self))
  (bind _output_get (set `self.WB_MainMenu` _returnvalue))
  (`UserWidget.AddToViewport` _output_get 0)
  (`self.SetupPlayerUI`))

(fn `Hide Loading Screen`
  (`/Game/GameBP/Blueprints/ClientMenu/UI/WB_MainMenu.Toggle Loading Screen` (`self.WB_MainMenu`) false))

(fn `SetupPlayerUI`
  (`/Game/GameBP/Blueprints/ClientMenu/UI/WB_MainMenu.SetupProfileUI` (`self.WB_MainMenu`) (`/Game/GameBP/Blueprints/ClientMenu/Objects/O_PlayerProfile.PlayerDisplayName` (`/Game/GameBP/Blueprints/GI_Core.PlayerProfile` (`self.GameInstRef`))))
  (`self.Event Update Player Coins`))

(fn `Show Loading Screen`
  (`/Game/GameBP/Blueprints/ClientMenu/UI/WB_MainMenu.Toggle Loading Screen` (`self.WB_MainMenu`) true))

(fn `UpdatePlayerCoinsUI`
  (params (GameResult :type "/Game/GameData/Data/Enums/E_GameResults Enum" :default "NewEnumerator0") (CoinReward :type Integer))
  (`/Game/GameBP/Blueprints/ClientMenu/UI/WB_MainMenu.ShowGameReward` (`self.WB_MainMenu`) GameResult CoinReward)
  (`self.Event Update Player Coins`))

(fn `UserConstructionScript`)