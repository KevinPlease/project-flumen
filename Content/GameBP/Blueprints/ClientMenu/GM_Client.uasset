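; Client menu game mode that runs PlayFab matchmaking and updates player coins after a match.
; On BeginPlay after a finished match, Cloud Script applies the result to the coin balance.
; Matchmaking checks coin eligibility, creates a size-based queue ticket with ping latency for a hardcoded region, then polls it by timer.
; A match yields server IP and port, joined after an onMatchFound Cloud Script call; errors display on the menu.
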(event `self.ReceiveBeginPlay`
  (bind _gameinstref (`self.GameInstRef`))
  ;[1 1 1] Begin Play
  (bind _asgi_core (cast `/Game/GameBP/Blueprints/GI_Core` (`GameplayStatics.GetGameInstance`)))
  (set `self.GameInstRef` _asgi_core)
  (bind _aspc_client (cast `/Game/GameBP/Blueprints/ClientMenu/PC_Client` (`GameplayStatics.GetPlayerController` 0)))
  (set `self.PlayerControllerRef` _aspc_client)
  (if (not (`/Game/GameBP/Blueprints/GI_Core.IsFirstTime` _gameinstref))
    (if (`|EnumInequality` (`/Game/GameBP/Blueprints/GI_Core.GameResult` _gameinstref) "NewEnumerator3")
      (`self.Event Update Coins`))
    (else
      (set `/Game/GameBP/Blueprints/GI_Core.IsFirstTime` false _gameinstref))))

(event `OnSuccess:UpdatePlayerCoins`
  (params (result :type "ClientExecuteCloudScriptResult Structure") (customData :type "Object Object Reference"))
  ;[1 1 1] Update Coins based on GameResult from latest match
  (bind _totalcoins (`/Game/GameBP/Blueprints/ClientMenu/Objects/O_PlayerProfile.SetCoins` (`/Game/GameBP/Blueprints/GI_Core.PlayerProfile` (`self.GameInstRef`)) (`KismetMathLibrary.FTrunc` (`PlayFabJsonValue.AsNumber` (`PlayFabJsonObject.GetField` (`.FunctionResult` (break `ClientExecuteCloudScriptResult` result)) "Value")))))
  (`/Game/GameBP/Blueprints/ClientMenu/PC_Client.UpdatePlayerCoinsUI` (`self.PlayerControllerRef`) _totalcoins)
  (set `/Game/GameBP/Blueprints/GI_Core.GameResult` "NewEnumerator3" (`self.GameInstRef`)) ; reset
)

(event `Event Update Coins`
  (bind _gameinstref (`self.GameInstRef`))
  ;[1 1 1] Update Coins based on GameResult from latest match
  (bind _outjson (`self.CreateTempJson`))
  (`PlayFabJsonObject.SetStringField` _outjson "gameResult" (`|GetEnumeratorNameAsString` (`/Game/GameBP/Blueprints/GI_Core.GameResult` _gameinstref)))
  (`PlayFabJsonObject.SetNumberField` _outjson "matchSize" (`KismetMathLibrary.Conv_IntToDouble` (`/Game/GameBP/Blueprints/GI_Core.Matchmaking Size` _gameinstref)))
  (`PlayFabClientAPI.ExecuteCloudScript` (make `ClientExecuteCloudScriptRequest` null "updatePlayerCoins" (`self.Json`)) (delegate `OnSuccess:UpdatePlayerCoins`) (delegate `OnFailure:UpdatePlayerCoins`)))

(event `OnFailure:UpdatePlayerCoins`
  (params (error :type "PlayFabError Structure") (customData :type "Object Object Reference"))
  ;[1 1 1] Update Coins based on GameResult from latest match
  (bind _errormsg (`/Game/GameBP/Blueprints/BPL_Utils.HandlePlayFabError` error))
  (`self.DEBUG_LogOnHUD` _errormsg true)
  (set `/Game/GameBP/Blueprints/GI_Core.GameResult` "NewEnumerator3" (`self.GameInstRef`)))

(event `OnSuccess:StartMatchmaking`
  (params (result :type "ClientExecuteCloudScriptResult Structure") (customData :type "Object Object Reference"))
  ;[1 1 1] Check if player can matchmake -- create the matchmaking ticket or report error
  (if (`PlayFabJsonValue.AsBool` (`PlayFabJsonObject.GetField` (`.FunctionResult` (break `ClientExecuteCloudScriptResult` result)) "Value"))
    (`self.CreateMatchmakingTicket` (`/Game/GameBP/Blueprints/ClientMenu/Objects/O_PlayerProfile.GetEntityId` (`/Game/GameBP/Blueprints/GI_Core.PlayerProfile` (`self.GameInstRef`))) (`self.GetQueueNameFromSize` (stale `StartMatchmaking` MatchSize)))
    (else
      (`self.DEBUG_LogOnHUD` "Not enough coins :(" true))))

(event `StartMatchmaking`
  (params (MatchSize :type Integer) (PlayerCoinFee :type Integer))
  (bind _json (`self.Json`))
  ;[1 1 1] Check if player can matchmake -- create the matchmaking ticket or report error
  (`/Game/GameBP/Blueprints/ClientMenu/PC_Client.Show Loading Screen` (`self.PlayerControllerRef`))
  (`self.CreateTempJson`)
  (`PlayFabJsonObject.SetNumberField` _json "playerMatchFee" (`KismetMathLibrary.Conv_IntToDouble` PlayerCoinFee))
  (`PlayFabClientAPI.ExecuteCloudScript` (make `ClientExecuteCloudScriptRequest` null "canMatchmake" _json) (delegate `OnSuccess:StartMatchmaking`) (delegate `OnFailure:StartMatchmaking`)))

(event `OnFailure:StartMatchmaking`
  (params (error :type "PlayFabError Structure") (customData :type "Object Object Reference"))
  ;[1 1 1] Check if player can matchmake -- create the matchmaking ticket or report error
  (bind _errormsg (`/Game/GameBP/Blueprints/BPL_Utils.HandlePlayFabError` error))
  (`self.DEBUG_LogOnHUD` _errormsg true))

(event `OnSuccess: CreateMatchmaking`
  (params (result :type "MultiplayerCreateMatchmakingTicketResult Structure") (customData :type "Object Object Reference"))
  (bind _intervaltocheckmatchstatus (`self.IntervalToCheckMatchStatus`))
  ;[1 1 1] Create the matchmaking rules and ticket
  (set `self.CurTicketId` (`.TicketId` (break `MultiplayerCreateMatchmakingTicketResult` result)))
  (bind _returnvalue (`KismetSystemLibrary.K2_SetTimer` null "CheckMatchStatus" _intervaltocheckmatchstatus true (* -1 _intervaltocheckmatchstatus)))
  (set `self.MatchFinderTimerHandle` _returnvalue))

(event `CreateMatchmakingTicket`
  (params (PlayerId :type String) (QueueName :type String))
  (bind _matchcreatesettings (`self.MatchCreateSettings`))
  ;[1 1 1] Create the matchmaking rules and ticket
  (set `self.CurQueueName` QueueName)
  (set `self.MatchCreateSettings` (`PlayFabJsonObject.ConstructJsonObject`))
  (bind _output_get (set `self.EntityKeySettings` (`PlayFabJsonObject.ConstructJsonObject`)))
  (`PlayFabJsonObject.SetStringField` _output_get "Id" PlayerId)
  (`PlayFabJsonObject.SetStringField` _output_get "Type" "title_player_account")
  (`PlayFabJsonObject.SetStringField` _output_get "TypeString" "title_player_account")
  (`PlayFabJsonObject.SetObjectField` _matchcreatesettings "Attributes" (`self.CreateMatchmakingAttributes`))
  (`PlayFabJsonObject.SetObjectField` _matchcreatesettings "Entity" (`self.EntityKeySettings`))
  (`PlayFabMultiplayerAPI.CreateMatchmakingTicket` (make `MultiplayerCreateMatchmakingTicketRequest` _matchcreatesettings null 60 (`|MakeArray`) (`self.CurQueueName`)) (delegate `OnSuccess: CreateMatchmaking`) (delegate `OnFail: CreateMatchmaking`)))

(event `OnFail: CreateMatchmaking`
  (params (error :type "PlayFabError Structure") (customData :type "Object Object Reference"))
  ;[1 1 1] Create the matchmaking rules and ticket
  (bind _errormsg (`/Game/GameBP/Blueprints/BPL_Utils.HandlePlayFabError` error))
  (`self.DEBUG_LogOnHUD` _errormsg true)
  (`KismetSystemLibrary.K2_ClearAndInvalidateTimerHandle` (`self.MatchFinderTimerHandle`)))

(event `OnSuccess: GetMatchmakingTicket`
  (params (result :type "MultiplayerGetMatchmakingTicketResult Structure") (customData :type "Object Object Reference"))
  (bind (_cancellationreasonstring _created _creator _giveupafterseconds _matchid _members _memberstomatchwith _queuename _status) (break `MultiplayerGetMatchmakingTicketResult` result))
  (bind _matchfindertimerhandle (`self.MatchFinderTimerHandle`))
  ;[1 1 1] Check matchmaking ticket status
  (switch `string` _status
    (:`Default`
      (`self.DEBUG_LogOnHUD` _status))
    (:`Matched`
      (`KismetSystemLibrary.K2_ClearAndInvalidateTimerHandle` _matchfindertimerhandle)
      (`self.GetMatch` _matchid _queuename))
    (:`Canceled`
      (`KismetSystemLibrary.K2_ClearAndInvalidateTimerHandle` _matchfindertimerhandle)
      (`self.DEBUG_LogOnHUD` "Matching timeout -- Try again" true))))

(event `GetMatchmakingTicket`
  (params (QueueName :type String) (TicketId :type String))
  ;[1 1 1] Check matchmaking ticket status
  (`PlayFabMultiplayerAPI.GetMatchmakingTicket` (make `MultiplayerGetMatchmakingTicketRequest` null false QueueName TicketId) (delegate `OnSuccess: GetMatchmakingTicket`) (delegate `OnFail: GetMatchmakingTicket`)))

(event `OnFail: GetMatchmakingTicket`
  (params (error :type "PlayFabError Structure") (customData :type "Object Object Reference"))
  ;[1 1 1] Check matchmaking ticket status
  (bind _errormsg (`/Game/GameBP/Blueprints/BPL_Utils.HandlePlayFabError` error))
  (`self.DEBUG_LogOnHUD` _errormsg true)
  (`KismetSystemLibrary.K2_ClearAndInvalidateTimerHandle` (`self.MatchFinderTimerHandle`)))

(event `OnSuccess: GetMatch`
  (params (result :type "MultiplayerGetMatchResult Structure") (customData :type "Object Object Reference"))
  (bind (_matchid _members _regionpreferences _serverdetails) (break `MultiplayerGetMatchResult` result))
  ;[1 1 1] Get Match details/server details -- connecto to server
  (bind _returnvalue (`PlayFabJsonObject.GetArrayField` _serverdetails "Ports"))
  (bind _returnvalue_2 (`PlayFabJsonValue.AsObject` (`|GetArrayItem` _returnvalue)))
  (`self.DEBUG_LogOnHUD` "Joining Match...")
  (set `/Game/GameBP/Blueprints/GI_Core.Matchmaking Size` (`KismetArrayLibrary.Array_Length` _members) (`self.GameInstRef`))
  (`self.Event Connect To Server` (`PlayFabJsonObject.GetStringField` _serverdetails "IPV4Address") (`KismetMathLibrary.FTrunc` (`PlayFabJsonObject.GetNumberField` _returnvalue_2 "Num"))))

(event `GetMatch`
  (params (MatchId :type String) (QueueName :type String))
  ;[1 1 1] Get Match details/server details -- connecto to server
  (`self.DEBUG_LogOnHUD` "Matched! Getting match info...")
  (`PlayFabMultiplayerAPI.GetMatch` (make `MultiplayerGetMatchRequest` null false MatchId QueueName) (delegate `OnSuccess: GetMatch`) (delegate `OnFail: GetMatch`)))

(event `OnFail: GetMatch`
  (params (error :type "PlayFabError Structure") (customData :type "Object Object Reference"))
  ;[1 1 1] Get Match details/server details -- connecto to server
  (bind _errormsg (`/Game/GameBP/Blueprints/BPL_Utils.HandlePlayFabError` error))
  (`self.DEBUG_LogOnHUD` _errormsg true))

(event `OnSuccess: ConnectToServer`
  (params (result :type "ClientExecuteCloudScriptResult Structure") (customData :type "Object Object Reference"))
  ;[1 1 1] Connect To Server: Call PlayFab event before joining the match
  (`/Game/GameBP/Blueprints/BPL_Utils.JoinServer` (`self.PlayerControllerRef`) (stale `Event Connect To Server` IP) (stale `Event Connect To Server` Port)))

(event `Event Connect To Server`
  (params (IP :type String) (Port :type Integer))
  ;[1 1 1] Connect To Server: Call PlayFab event before joining the match
  (`PlayFabClientAPI.ExecuteCloudScript` (make `ClientExecuteCloudScriptRequest` null "onMatchFound") (delegate `OnSuccess: ConnectToServer`) (delegate `OnFailure: ConnectToServer`)))

(event `OnFailure: ConnectToServer`
  (params (error :type "PlayFabError Structure") (customData :type "Object Object Reference"))
  ;[1 1 1] Connect To Server: Call PlayFab event before joining the match
  (bind _errormsg (`/Game/GameBP/Blueprints/BPL_Utils.HandlePlayFabError` error))
  (`self.DEBUG_LogOnHUD` _errormsg true))

(fn `CheckMatchStatus`
  (bind _curticketid (`self.CurTicketId`))
  (`self.GetMatchmakingTicket` (`self.CurQueueName`) _curticketid)
  (`self.DEBUG_LogOnHUD` (`KismetStringLibrary.Concat_StrStr` "Searching match with id: " _curticketid)))

(fn `CreateMatchmakingAttributes`
  (returns (MatchmakingAttrs :type "PlayFabJsonObject Object Reference"))
  (locals (Region :type "PlayFabJsonObject Object Reference") (DataObject :type "PlayFabJsonObject Object Reference") (Attributes :type "PlayFabJsonObject Object Reference"))
  (bind _output_get (set `local.Region` (`PlayFabJsonObject.ConstructJsonObject`)))
  (`PlayFabJsonObject.SetStringField` _output_get "region" "NorthEurope")
  (`PlayFabJsonObject.SetNumberField` _output_get "latency" (`KismetMathLibrary.Conv_ByteToDouble` (`PlayerState.Ping` (`Controller.PlayerState` (`self.PlayerControllerRef`)))))
  (bind _output_get_2 (set `local.DataObject` (`PlayFabJsonObject.ConstructJsonObject`)))
  (`PlayFabJsonObject.SetObjectArrayField` _output_get_2 "Latencies" (`|MakeArray` (`local.Region`)))
  (bind _output_get_3 (set `local.Attributes` (`PlayFabJsonObject.ConstructJsonObject`)))
  (`PlayFabJsonObject.SetObjectField` _output_get_3 "DataObject" (`local.DataObject`))
  (return (`local.Attributes`)))

(fn `CreateTempJson`
  (returns (OutJson :type "PlayFabJsonObject Object Reference"))
  (bind _output_get (set `self.Json` (`PlayFabJsonObject.ConstructJsonObject`)))
  (return _output_get))

(fn `DEBUG_LogOnHUD`
  (params (Message :type String) (IsError :type Boolean))
  (bind _playercontrollerref (`self.PlayerControllerRef`))
  (bind _wb_mainmenu (`/Game/GameBP/Blueprints/ClientMenu/PC_Client.WB_MainMenu` _playercontrollerref))
  (if IsError
    (`/Game/GameBP/Blueprints/ClientMenu/UI/WB_MainMenu.SetError` _wb_mainmenu Message)
    (`/Game/GameBP/Blueprints/ClientMenu/UI/WB_MainMenu.SetStatus` _wb_mainmenu "Error")
    (`/Game/GameBP/Blueprints/ClientMenu/PC_Client.Hide Loading Screen` _playercontrollerref)
    (`/Game/GameBP/Blueprints/ClientMenu/UI/WB_MainMenu.ShowMenu` _wb_mainmenu "NewEnumerator1")
    (else
      (`/Game/GameBP/Blueprints/ClientMenu/UI/WB_MainMenu.SetStatus` _wb_mainmenu Message))))

(fn `GetQueueNameFromSize`
  (params (MatchSize :type Integer))
  (returns (QueueName :type String))
  (switch `int` MatchSize
    (:`2`
      (return "1v1"))
    (:`3`
      (return "ThreePeeps"))
    (:`4`
      (return "FourPeeps"))))

(fn `UserConstructionScript`)